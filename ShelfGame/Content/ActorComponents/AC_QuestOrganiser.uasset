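; Actor component that tracks active and finished quests for its owner and drives the quest tracker widget.
; On BeginPlay it creates a hidden tracker UI, then spawns and adds a BP_CollectBlueprint quest; an input action toggles the log.
; Quests are keyed by gameplay tag in two maps, rejecting duplicates when added.
; AddQuest starts each quest and binds its update and completion events; CompleteQuest moves it to finished and refreshes the UI.
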(event `self.ReceiveBeginPlay`
  (bind _returnvalue (`|CreateWidget` "/Game/Quests/Widgets/WBP_QuestTracker.WBP_QuestTracker_C" (`GameplayStatics.GetPlayerController` 0) self))
  (bind _output_get (set `self.Quest UI` _returnvalue))
  (`UserWidget.AddToViewport` _output_get 0)
  (`Widget.SetVisibility` _output_get "Collapsed")
  (bind _returnvalue_2 (`|SpawnActorFromClass` "/Game/Quests/Quests/BP_CollectBlueprint.BP_CollectBlueprint_C" (`Actor.GetTransform` (`self.GetOwner`)) "AlwaysSpawn" "MultiplyWithRoot" null null))
  (`self.Add Quest` _returnvalue_2)
  (`/Game/Quests/Widgets/WBP_QuestTracker.Update Quest Lists` _output_get))

(event `EnhancedInput|/Game/Characters/Player/Input/Actions/IA_ShowQuestLog`
  (params (ActionValue :type Boolean) (ElapsedSeconds :type "Float (double-precision)") (TriggeredSeconds :type "Float (double-precision)") (InputAction :type "InputAction Object Reference" :default "/Game/Characters/Player/Input/Actions/IA_ShowQuestLog.IA_ShowQuestLog"))
  (:`Triggered`
    (`/Game/Quests/Widgets/WBP_QuestTracker.Toggle Quest Tracker Visability` (`self.Quest UI`))))

(fn `Add Quest`
  (params (`Quest To Add` :type "/Game/Quests/Quests/BP_BaseQuest Object Reference"))
  (if (and (not (`self.IsQuestActive` `Quest To Add`)) (not (`self.IsQuestFinished` `Quest To Add`)))
    (`BlueprintMapLibrary.Map_Add` (`self.Active Quests`) (`/Game/Quests/Quests/BP_BaseQuest.QuestID` `Quest To Add`) `Quest To Add`)
    (add `/Game/Quests/Quests/BP_BaseQuest.Quest Updated` `Quest To Add` (`|CreateDelegate` :!event `Update Quest UI`))
    (`/Game/Quests/Quests/BP_BaseQuest.Start Quest` `Quest To Add`)
    (add `/Game/Quests/Quests/BP_BaseQuest.Completed Quest` `Quest To Add` (`|CreateDelegate` :!event `Complete Quest`))
    (`KismetSystemLibrary.PrintString` (`KismetTextLibrary.Conv_TextToString` (`|FormatText` "{Quest} Is now active" (`BlueprintGameplayTagLibrary.GetDebugStringFromGameplayTag` (`/Game/Quests/Quests/BP_BaseQuest.QuestID` `Quest To Add`)))))))

(fn `Complete Quest`
  (params (`Completed Quest` :type "/Game/Quests/Quests/BP_BaseQuest Object Reference"))
  (bind _questid (`/Game/Quests/Quests/BP_BaseQuest.QuestID` `Completed Quest`))
  (`BlueprintMapLibrary.Map_Remove` (`self.Active Quests`) _questid)
  (`BlueprintMapLibrary.Map_Add` (`self.Finished Quests`) _questid `Completed Quest`)
  (`/Game/Quests/Widgets/WBP_QuestTracker.Update Quest Lists` (`self.Quest UI`)))

(fn `Get Specific Active Quest`
  (params (`Quest ID` :type "GameplayTag Structure"))
  (returns (Quest :type "/Game/Quests/Quests/BP_BaseQuest Object Reference") (`Quest Found` :type Boolean))
  (bind (_value _returnvalue) (`BlueprintMapLibrary.Map_Find` (`self.Active Quests`) `Quest ID`))
  (return _value _returnvalue))

(fn `IsQuestActive`
  (params (`Quest To Check` :type "/Game/Quests/Quests/BP_BaseQuest Object Reference"))
  (returns (QuestActive :type Boolean))
  (return (`BlueprintMapLibrary.Map_Contains` (`self.Active Quests`) (`/Game/Quests/Quests/BP_BaseQuest.QuestID` `Quest To Check`))))

(fn `IsQuestFinished`
  (params (`Quest To Check` :type "/Game/Quests/Quests/BP_BaseQuest Object Reference"))
  (returns (QuestFinished :type Boolean))
  (return (`BlueprintMapLibrary.Map_Contains` (`self.Finished Quests`) (`/Game/Quests/Quests/BP_BaseQuest.QuestID` `Quest To Check`))))

(fn `Update Quest UI`
  (`/Game/Quests/Widgets/WBP_QuestTracker.Update Quest Lists` (`self.Quest UI`)))