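; Actor component that manages the player's tool inventory and the gameplay ability tied to each tool.
; On BeginPlay it adds an AbilitySystemComponent to its owner, creates the selection widget and grants an invisible default pickup tool.
; Gained tools attach to the skeletal mesh socket and grant their ability; equipping swaps visibility and the active tag, which the use input activates.
; Re-triggering the Pickup ability drops held actors when switching to another tool.
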(event `self.ReceiveBeginPlay`
  (bind _tool_selection_widget (`self.Tool Selection Widget`))
  ; Give the owner an ability system component
  (bind _returnvalue (`|AddComponentByClass` (`self.GetOwner`) "/Script/GameplayAbilities.AbilitySystemComponent"))
  (set `self.Ability System` _returnvalue)
  ; Create Tool Selection Widget
  (bind _returnvalue_2 (`|CreateWidget` "/Game/Tools/ToolSelectionWidgets/WBP_ToolInventory.WBP_ToolInventory_C" (`GameplayStatics.GetPlayerController` 0)))
  (bind _output_get (set `self.Tool Selection Widget` _returnvalue_2))
  (add `/Game/Tools/ToolSelectionWidgets/WBP_ToolInventory.Tool Selected` _output_get (`|CreateDelegate` :!event `Use New Tool Selected From Inventory`))
  (`UserWidget.AddToViewport` _tool_selection_widget 0)
  (set `Widget.Visibility` "Collapsed" _tool_selection_widget)
  ; Creates the pickup tool which is an invisible tool that allows you to pickup actors
  (bind _returnvalue_3 (`|SpawnActorFromClass` "/Game/Tools/ToolActors/BP_Tools_Pickup.BP_Tools_Pickup_C" (`Actor.GetTransform` (`self.GetOwner`)) "Undefined" "MultiplyWithRoot" null null))
  (bind _output_get_2 (set `self.Pickup Tool` _returnvalue_3))
  (`self.Gain Tool` _output_get_2)
  (add `self.Tool Equipped` (`|CreateDelegate` :!event `Drop Held Actor`)))

(event `Gain Tool`
  (params (`Gained Tool` :type "/Game/Tools/ToolActors/BP_ToolsBase Object Reference"))
  (bind _returnvalue (`KismetSystemLibrary.IsValid` `Gained Tool`))
  (bind (_toolimage _toolabilitytag _toolabilityclass) (break `/Game/Tools/ToolSelectionWidgets/F_ToolInformation` (`/Game/Tools/ToolActors/BP_ToolsBase.Tool Information` `Gained Tool`)))
  ; When interacted with a tool, gain the ability and equip it from the interact interface
  (`KismetSystemLibrary.PrintString` (`KismetTextLibrary.Conv_TextToString` (`|FormatText` "Is Pickup Tool Successful - {bool}" _returnvalue)) true true (struct :`G` 0.66 :`B` 1.0 :`A` 1.0) 3.0)
  (if _returnvalue
    (`KismetArrayLibrary.Array_AddUnique` (`self.Gained Tools`) `Gained Tool`)
    (`/Game/Tools/ToolSelectionWidgets/WBP_ToolInventory.Add Tool To Inventory` (`self.Tool Selection Widget`) `Gained Tool`)
    (`self.SetCurrentToolAndAbility` `Gained Tool` _toolabilitytag)
    (`AbilitySystemComponent.K2_GiveAbility` (`self.Ability System`) _toolabilityclass 0 -1)
    (bind _returnvalue_2 (`Actor.K2_AttachToComponent` `Gained Tool` (`Actor.GetComponentByClass` (`self.GetOwner`) "/Script/Engine.SkeletalMeshComponent") (`self.Socket To Attach Tool`) "SnapToTarget" "SnapToTarget" "SnapToTarget" true))
    (bind _output_get (set `/Game/Tools/ToolActors/BP_ToolsBase.Has Been Picked Up` _returnvalue_2 `Gained Tool`))
    (if _output_get
      (`Actor.SetActorEnableCollision` `Gained Tool` false)
      (`KismetSystemLibrary.PrintString` "Tool Attached To Actor" true true (struct :`G` 1.0 :`B` 0.039869 :`A` 1.0) 3.0)
      (else
        (`KismetSystemLibrary.PrintString` "FAILED TO ATTACH TOOL TO ACTOR" true true (struct :`R` 1.0 :`B` 0.024311 :`A` 1.0) 10.0)))))

(event `Display Tool Inventory`
  (bind _tool_selection_widget (`self.Tool Selection Widget`))
  ; Display The Tool Inventory
  (if (not (<= (`KismetArrayLibrary.Array_Length` (`self.Gained Tools`)) 1))
    (`/Engine/EditorBlueprintResources/StandardMacros.IsValid` _tool_selection_widget
      (:`Is Valid`
        (`Widget.SetVisibility` _tool_selection_widget "SelfHitTestInvisible")
        (`/Game/FunctionLibraries/BPI_UIFunctions.SetMouseCursorToCenter`)
        (message `/Game/Interfaces/BPI_ToggleInputForDialogue.Toggle Input` (`GameplayStatics.GetPlayerController` 0) false false true)))))

(event `Use New Tool Selected From Inventory`
  (params (`Selected Tool` :type "/Game/Tools/ToolActors/BP_ToolsBase Object Reference") (`Ability Tag` :type "GameplayTagContainer Structure"))
  (bind _tool_selection_widget (`self.Tool Selection Widget`))
  ; When a Tool Is selected from the inventory, equip the tool
  (`self.SetCurrentToolAndAbility` `Selected Tool` `Ability Tag`)
  (`/Engine/EditorBlueprintResources/StandardMacros.IsValid` _tool_selection_widget
    (:`Is Valid`
      (set `Widget.Visibility` "Collapsed" _tool_selection_widget))
    (:`Is Not Valid`
      (`KismetSystemLibrary.PrintString` "Tool Selection Widget within AC_ToolInventoryAndAbilities Not Valid" true true (struct :`R` 1.0 :`G` 0.022888 :`A` 1.0) 10.0)))
  (message `/Game/Interfaces/BPI_ToggleInputForDialogue.Toggle Input` (`GameplayStatics.GetPlayerController` 0) true true false))

(event `EnhancedInput|/Game/Characters/Player/Input/Actions/IA_UseAbility`
  (params (ActionValue :type Boolean) (ElapsedSeconds :type "Float (double-precision)") (TriggeredSeconds :type "Float (double-precision)") (InputAction :type "InputAction Object Reference" :default "/Game/Characters/Player/Input/Actions/IA_UseAbility.IA_UseAbility"))
  (bind _current_ability (`self.Current Ability`))
  ; Use the current ability that is equiped
  (:`Triggered`
    (bind _returnvalue (`AbilitySystemComponent.TryActivateAbilitiesByTag` (`self.Ability System`) _current_ability true))
    (`KismetSystemLibrary.PrintString` (`KismetTextLibrary.Conv_TextToString` (`|FormatText` "Ability - {ability}. Successfull - {successfull}" (`BlueprintGameplayTagLibrary.GetDebugStringFromGameplayTagContainer` _current_ability) _returnvalue)) true true (struct :`G` 0.66 :`B` 1.0 :`A` 1.0) 2.0 "Ability Successfull ")))

(event `Drop Held Actor`
  ; Drop the held actor if the new tool isnt the pickup tool
  (bind _bsuccess (message `/Game/Interfaces/BPI_GetFromPlayer.Get Held Object` (`self.GetOwner`)))
  (if (and _bsuccess (!= (`self.Current Ability`) (`BlueprintGameplayTagLibrary.MakeLiteralGameplayTagContainer` (struct :`GameplayTags` (struct :`(TagName` "Ability.Pickup"))))))
    (`AbilitySystemComponent.TryActivateAbilitiesByTag` (`self.Ability System`) (`BlueprintGameplayTagLibrary.MakeLiteralGameplayTagContainer` (struct :`GameplayTags` (struct :`(TagName` "Ability.Pickup")))) true)))

(fn `SetCurrentToolAndAbility`
  (params (Tool :type "/Game/Tools/ToolActors/BP_ToolsBase Object Reference") (`Ability Tag` :type "GameplayTagContainer Structure"))
  (`/Engine/EditorBlueprintResources/StandardMacros.IsValid` Tool
    (:`Is Valid`
      (bind _current_tool (`self.Current Tool`)
        (:`then`
          (if (not (== Tool _current_tool))
            (`Actor.SetActorHiddenInGame` _current_tool true)
            (`Actor.SetActorHiddenInGame` Tool false :!label _label)
            (set `self.Current Tool` Tool)
            (set `self.Current Ability` `Ability Tag`)
            (`self.Tool Equipped`)))
        (:`else`
          (goto _label))))
    (:`Is Not Valid`
      _))
  (`KismetSystemLibrary.PrintString` (`KismetTextLibrary.Conv_TextToString` (`|FormatText` "New Tool - {Tool} \nNew Ability - {Ability}" (`self.Current Tool`) (`BlueprintGameplayTagLibrary.GetDebugStringFromGameplayTagContainer` (`self.Current Ability`)))) true true (struct :`G` 0.66 :`B` 1.0 :`A` 1.0) 5.0 "PickUp Tool"))