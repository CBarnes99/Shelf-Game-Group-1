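; Actor component that shifts its owner between depth planes along the Y axis.
; CanActorPivot rejects moves mid-pivot, past the end planes or blocked by a sphere trace, except BPI_LineClimb hits, which get a ClimbTheLine message.
; Accepted pivots update the plane and distance, then looping timers lerp only Y along a float curve until a short timer ends it.
; PivotPlayerJump separately makes player-tagged characters jump at pivot velocity, restoring the default on landing.
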(event `Start Pivot`
  (set `self.Actor Starting Loc` (`Actor.K2_GetActorLocation` (`self.GetOwner`)))
  (set `self.Currently Pivoting` true)
  (bind _returnvalue (`KismetSystemLibrary.K2_SetTimerDelegate` (`|CreateDelegate` :!event `Finish Pivot`) 0.2))
  (bind _returnvalue_2 (`KismetSystemLibrary.K2_SetTimerDelegate` (`|CreateDelegate` :!event `Update Location`) 0.005 true)))

(event `Update Location`
  (bind _returnvalue (`self.GetOwner`))
  (bind _actor_starting_loc (`self.Actor Starting Loc`))
  (bind (_returnvalue_x _returnvalue_y _returnvalue_z) (`KismetMathLibrary.BreakVector` (`Actor.K2_GetActorLocation` _returnvalue)))
  (bind (_returnvalue_x_2 _returnvalue_y_2) (`KismetMathLibrary.BreakVector` (`KismetMathLibrary.VLerp` _actor_starting_loc (+ _actor_starting_loc (`KismetMathLibrary.MakeVector` 0.0 (`self.Direction and Distance`))) (`KismetMathLibrary.GetRuntimeFloatCurveValue` (`self.Curve`) (`KismetSystemLibrary.K2_GetTimerElapsedTimeHandle` (stale `Start Pivot` _returnvalue))))))
  (`Actor.K2_SetActorLocation` _returnvalue (`KismetMathLibrary.MakeVector` _returnvalue_x _returnvalue_y_2 _returnvalue_z) false false))

(event `Finish Pivot`
  (set `self.Currently Pivoting` false)
  (`KismetSystemLibrary.K2_ClearAndInvalidateTimerHandle` (stale `Start Pivot` _returnvalue_2)))

(fn `Can Actor Pivot`
  (params (Direction :type "Float (double-precision)"))
  (returns (bSuccess :type Boolean))
  (locals (IsPivotNotBlocked :type Boolean :default false))
  (bind _current_plane (`self.Current Plane`))
  (if (not (`self.Currently Pivoting`))
    (bind _babletopivot (`self.Trace Direction` (`Actor.K2_GetActorLocation` (`self.GetOwner`)) Direction))
    (set `local.IsPivotNotBlocked` _babletopivot)
    (if (< Direction 0.0)
      (if (and (not (== (`self.Current Plane`) (`self.Amount of Planes`))) (`local.IsPivotNotBlocked`))
        (`/Engine/EditorBlueprintResources/StandardMacros.IncrementInt` _current_plane
          (:`  `
            _))
        (else
          (`KismetSystemLibrary.PrintString` "Already In Back" true true (struct :`G` 0.66 :`B` 1.0 :`A` 1.0) 2.0 "Pivot")
          (return false)))
      (elif (and (`local.IsPivotNotBlocked`) (not (== (`self.Current Plane`) 1)))
        (`/Engine/EditorBlueprintResources/StandardMacros.DecrementInt` (`self.Current Plane`)
          (:`  `
            _))
        (else
          (`KismetSystemLibrary.PrintString` "Already In Front" true true (struct :`G` 0.66 :`B` 1.0 :`A` 1.0) 2.0 "Pivot")
          (return false))))
    (set `self.Current Plane` (`KismetMathLibrary.Clamp` _current_plane 1 (`self.Amount of Planes`)))
    (`self.Set Distance to Pivot`)
    ; Negative = Back a plane. Positive = Forward a plane.
    (set `self.Direction and Distance` (* Direction (`self.Distance To Pivot`)))
    (`self.Start Pivot`)
    (return true)
    (else
      (`KismetSystemLibrary.PrintString` "Currently Pivoting" true true (struct :`G` 0.66 :`B` 1.0 :`A` 1.0) 2.0 "Pivoting"))))

(fn `PivotPlayerJump`
  (bind _returnvalue (`self.GetOwner`))
  (bind _player (`self.Player`))
  (bind _ascharacter (cast `Character` _returnvalue))
  (if (and (`KismetSystemLibrary.IsValid` _ascharacter) (`Actor.ActorHasTag` _returnvalue "Player"))
    (`|ExecutionSequence`
      (:`then_0`
        (`/Engine/EditorBlueprintResources/StandardMacros.DoOnce` false
          (:`Completed`
            (bind _output_get (set `self.Player` _ascharacter))
            (set `self.Default Jump Z Velocity` (`CharacterMovementComponent.JumpZVelocity` (`Character.CharacterMovement` _output_get))))))
      (:`then_1`
        (if (not (`NavMovementInterface.IsFalling` (`Character.CharacterMovement` (`self.Player`))))
          (set `CharacterMovementComponent.JumpZVelocity` (`self.Pivot Jump Velocity`) (`Character.CharacterMovement` _player))
          (`Character.Jump` _player)
          (bind _returnvalue_2 (`KismetSystemLibrary.K2_SetTimer` null "StopJumping" 0.01 true))
          (set `self.Jumping Timer` _returnvalue_2))))))

(fn `Set Distance to Pivot`
  (bind (_returnvalue_x _returnvalue_y) (`KismetMathLibrary.BreakVector` (`Actor.K2_GetActorLocation` (`self.GetOwner`))))
  (bind (_output_x _output_y) (`KismetMathLibrary.BreakVector` (`|GetArrayItem` (`self.Plane Y Locations`) (- (`self.Current Plane`) 1))))
  (set `self.Distance To Pivot` (`KismetMathLibrary.Abs` (- _returnvalue_y _output_y))))

(fn `Set Pivot Radius`
  (params (`Radius of Pivot Check` :type "Float (double-precision)"))
  (set `self.Radius of Pivot Check` `Radius of Pivot Check`))

(fn `Set Plane Information`
  (params (`Current Plane` :type Integer) (`Amount of Planes` :type Integer) (`Plane Y Locs` :type "Array of Vector Structure"))
  (set `self.Current Plane` `Current Plane`)
  (set `self.Amount of Planes` `Amount of Planes`)
  (set `self.Plane Y Locations` `Plane Y Locs`))

(fn `StopJumping`
  (bind _player (`self.Player`))
  (if (not (`NavMovementInterface.IsFalling` (`Character.CharacterMovement` (`self.Player`))))
    (`KismetSystemLibrary.K2_ClearAndInvalidateTimerHandle` (`self.Jumping Timer`))
    (`Character.StopJumping` _player)
    (set `CharacterMovementComponent.JumpZVelocity` (`self.Default Jump Z Velocity`) (`Character.CharacterMovement` _player))))

(fn `Trace Direction`
  (params (`Starting Loc` :type "Vector Structure") (Direction :type "Float (double-precision)"))
  (returns (bAbleToPivot :type Boolean))
  (bind (_outhit _returnvalue) (`KismetSystemLibrary.SphereTraceSingle` :`Start` `Starting Loc` :`End` (+ `Starting Loc` (`KismetMathLibrary.MakeVector` 0.0 (* Direction (`self.Distance To Pivot`)))) :`Radius` (`self.Radius of Pivot Check`) :`TraceChannel` "TraceTypeQuery1" :`DrawDebugType` "ForDuration" :`DrawTime` 1.0))
  (if _returnvalue
    (bind (_bblockinghit _binitialoverlap _time _distance _location _impactpoint _normal _impactnormal _physmat _hitactor) (`GameplayStatics.BreakHitResult` _outhit))
    (if (`KismetSystemLibrary.DoesImplementInterface` _hitactor "/Game/Interfaces/BPI_LineClimb.BPI_LineClimb_C")
      (message `/Game/Interfaces/BPI_LineClimb.Climb The Line` _hitactor)
      (return true)
      (else
        (return false)))
    (else
      (return (not _returnvalue)))))