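; Actor component that lets a tagged player push or pull its owner a set distance along the X axis.
; The owner's box overlaps track player range, and line traces in CanPush check that the path is clear.
; A move attaches the player, disables input and sweeps the owner along a timer-driven curve lerp, stopping on blocking hits.
; PivotObject delegates pivot checks to the owner's AC_PivotBetweenPlanes.
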(event `self.ReceiveBeginPlay`
  (bind _returnvalue (`Actor.GetComponentByClass` (`self.GetOwner`) "/Script/Engine.BoxComponent"))
  (`/Engine/EditorBlueprintResources/StandardMacros.IsValid` _returnvalue
    (:`Is Valid`
      (set `self.Box Collision` _returnvalue)
      (add `PrimitiveComponent.OnComponentBeginOverlap` _returnvalue (`|CreateDelegate` :!event `On Overlap Begin`))
      (add `PrimitiveComponent.OnComponentEndOverlap` _returnvalue (`|CreateDelegate` :!event `On Overlap Ends`)))
    (:`Is Not Valid`
      (`KismetSystemLibrary.PrintString` (`KismetTextLibrary.Conv_TextToString` (`|FormatText` "{owner} donest have box collision for AC_PushableObject!" (`self.GetOwner`)))))))

(event `Push Cube Called From Owner`
  (params (Direction :type "Float (double-precision)") (Player :type "Character Object Reference"))
  (bind _player (`self.Player`))
  (bind _output_get (set `self.Direction` Direction))
  (`|ExecutionSequence`
    (:`then_0`
      (`/Engine/EditorBlueprintResources/StandardMacros.DoOnce` false
        (:`Completed`
          (set `self.Player` Player))))
    (:`then_1`
      (if (`Actor.ActorHasTag` (`self.Player`) "Player")
        (set `self.PushableDirection` (`KismetMathLibrary.MakeVector` _output_get))
        (bind _canpush (`self.Can Push` _output_get _player))
        (if _canpush
          (`Actor.K2_AttachToActor` _player (`self.GetOwner`) "None" "KeepWorld" "KeepWorld" "KeepWorld" true)
          (`self.Push`))))))

(event `Push`
  (set `self.CurrentLocation` (`Actor.K2_GetActorLocation` (`self.GetOwner`)))
  (message `/Game/Interfaces/BPI_ToggleInputForDialogue.Toggle Input` (`GameplayStatics.GetPlayerController` 0) false true false)
  (bind _returnvalue (`KismetSystemLibrary.K2_SetTimerDelegate` (`|CreateDelegate` :!event `Stop Pushing`) 0.01))
  (bind _returnvalue_2 (`KismetSystemLibrary.K2_SetTimerDelegate` (`|CreateDelegate` :!event `Start Pushing`) 0.0001 true)))

(event `Start Pushing`
  (bind _returnvalue (`self.GetOwner`))
  (bind _currentlocation (`self.CurrentLocation`))
  (bind (_returnvalue_x _returnvalue_y _returnvalue_z) (`KismetMathLibrary.BreakVector` (`Actor.K2_GetActorLocation` _returnvalue)))
  (bind _returnvalue_x_2 (`KismetMathLibrary.BreakVector` (`KismetMathLibrary.VLerp` _currentlocation (+ _currentlocation (`KismetMathLibrary.MakeVector` (* (`self.TravelDistance`) (`self.Direction`)) (.y _currentlocation) (.z _currentlocation))) (`KismetMathLibrary.GetRuntimeFloatCurveValue` (`self.Curve`) (`KismetSystemLibrary.K2_GetTimerElapsedTimeHandle` (stale `Push` _returnvalue))))))
  (bind _sweephitresult (`Actor.K2_SetActorLocation` _returnvalue (`KismetMathLibrary.MakeVector` _returnvalue_x_2 _returnvalue_y _returnvalue_z) true false))
  (bind (_bblockinghit _binitialoverlap _time _distance _location _impactpoint _normal _impactnormal _physmat _hitactor) (`GameplayStatics.BreakHitResult` _sweephitresult))
  (if (and _bblockinghit (!= _hitactor (`self.Player`)))
    (`self.Stop Pushing`)))

(event `Stop Pushing`
  (`Actor.K2_DetachFromActor` (`self.Player`) "KeepWorld" "KeepWorld" "KeepWorld")
  (message `/Game/Interfaces/BPI_ToggleInputForDialogue.Toggle Input` (`GameplayStatics.GetPlayerController` 0) true true false)
  (`KismetSystemLibrary.K2_InvalidateTimerHandle` (stale `Push` _returnvalue_2))
  (`KismetSystemLibrary.K2_InvalidateTimerHandle` (stale `Push` _returnvalue)))

(event `On Overlap Begin`
  (params (OverlappedComponent :type "PrimitiveComponent Object Reference") (OtherActor :type "Actor Object Reference") (OtherComp :type "PrimitiveComponent Object Reference") (OtherBodyIndex :type Integer) (bFromSweep :type Boolean) (SweepResult :type "HitResult Structure (by ref)"))
  (if (`Actor.ActorHasTag` OtherActor "Player")
    (set `self.PlayerInRange` true)
    (`KismetSystemLibrary.PrintString` (`KismetTextLibrary.Conv_TextToString` (`|FormatText` "Player In Range To Push = {bool}" (`self.PlayerInRange`))) :!label _label)))

(event `On Overlap Ends`
  (params (OverlappedComponent :type "PrimitiveComponent Object Reference") (OtherActor :type "Actor Object Reference") (OtherComp :type "PrimitiveComponent Object Reference") (OtherBodyIndex :type Integer))
  (if (`Actor.ActorHasTag` OtherActor "Player")
    (set `self.PlayerInRange` false)
    (goto _label)))

(fn `Can Push`
  (params (Direction :type "Float (double-precision)") (Player :type "Character Object Reference"))
  (returns (CanPush :type Boolean))
  (bind _returnvalue (`Actor.K2_GetActorLocation` Player))
  (bind _player (`local.Player`))
  (bind _direction (`local.Direction`))
  (bind _returnvalue_2 (`Actor.K2_GetActorLocation` _player))
  (bind _boxextent_x (`KismetMathLibrary.BreakVector` (`BoxComponent.BoxExtent` (`self.Box Collision`))))
  (bind _returnvalue_3 (+ (`Actor.K2_GetActorLocation` (`self.GetOwner`)) (`KismetMathLibrary.MakeVector` (* _boxextent_x _direction))))
  ; Check to see if the push object is in front of the player
  (bind _outhit (`KismetSystemLibrary.LineTraceSingle` _returnvalue (+ _returnvalue (* (`KismetMathLibrary.SelectVector` (-1.0 0.0 0.0) (1.0 0.0 0.0) (< Direction 0.0)) (+ (`self.TravelDistance`) 100.0))) "TraceTypeQuery1" false (`|MakeArray` Player :!type "Actor Object Reference") "ForOneFrame" false))
  (bind (_bblockinghit _binitialoverlap _time _distance _location _impactpoint _normal _impactnormal _physmat _hitactor) (`GameplayStatics.BreakHitResult` _outhit))
  (`KismetSystemLibrary.PrintString` (`KismetTextLibrary.Conv_TextToString` (`|FormatText` "Hit Actor- {a}" _hitactor)) true true (struct :`G` 0.66 :`B` 1.0 :`A` 1.0) 100.0 "hit")
  (if (and _bblockinghit (== _hitactor (`self.GetOwner`)))
    ; If the Push block is in the direction of movement, do a line trace from the edge of the push block to see if its colliding
    (bind (_outhit_2 _returnvalue_4) (`KismetSystemLibrary.LineTraceSingle` :`Start` _returnvalue_3 :`End` (+ _returnvalue_3 (* (`self.TravelDistance`) _direction)) :`TraceChannel` "TraceTypeQuery1" :`DrawDebugType` "ForDuration" :`DrawTime` 1.0))
    (if _returnvalue_4
      (return false)
      (else
        (return true)))
    (else
      ; If the push block is not in the direction of movement, do a line trace from the player
      (bind (_outhit_3 _returnvalue_5) (`KismetSystemLibrary.LineTraceSingle` _returnvalue_2 (+ _returnvalue_2 (* (`KismetMathLibrary.SelectVector` (-1.0 0.0 0.0) (1.0 0.0 0.0) (< (`local.Direction`) 0.0)) (+ (`self.TravelDistance`) 20.0))) "TraceTypeQuery1" false (`|MakeArray` _player :!type "Actor Object Reference") "ForDuration" true (struct :`R` 1.0 :`A` 1.0) (struct :`G` 1.0 :`A` 1.0) 1.0))
      (if _returnvalue_5
        (return false)
        (else
          (return true))))))

(fn `isPlayerInRangeAndAbleToPush`
  (returns (PlayerAbleToPush :type Boolean))
  (return (and (`self.PlayerInRange`) (`self.AbleToPush`))))

(fn `Pivot Object`
  (params (Direction :type "Float (double-precision)"))
  (returns (bSuccess :type Boolean))
  (bind _returnvalue (`Actor.GetComponentByClass` (`self.GetOwner`) "/Game/ActorComponents/AC_PivotBetweenPlanes.AC_PivotBetweenPlanes_C"))
  (`/Engine/EditorBlueprintResources/StandardMacros.IsValid` _returnvalue
    (:`Is Valid`
      (bind _bsuccess (`/Game/ActorComponents/AC_PivotBetweenPlanes.Can Actor Pivot` _returnvalue Direction))
      (return _bsuccess))
    (:`Is Not Valid`
      (`KismetSystemLibrary.PrintString` "Owner doenst pivot")
      (return false))))