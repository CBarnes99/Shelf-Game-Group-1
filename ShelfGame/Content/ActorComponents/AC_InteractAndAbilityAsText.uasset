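; Interact prompt component that chooses which key to show the player as text, based on the held object or equipped tool.
; A held tin pickup yields the parent's interact key, while other held objects yield none.
; Otherwise, a current tool matching the configured class yields the key mapped to the use-ability input action.
; Extends the parent's overlap show/hide with a looping half-second timer that runs while the player overlaps.
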(event `self.Show Widget`
  (params (OverlappedComponent :type "PrimitiveComponent Object Reference") (OtherActor :type "Actor Object Reference") (OtherComp :type "PrimitiveComponent Object Reference") (OtherBodyIndex :type Integer) (bFromSweep :type Boolean) (SweepResult :type "HitResult Structure (by ref)"))
  (`parent.Show Widget` OverlappedComponent OtherActor OtherComp OtherBodyIndex bFromSweep SweepResult)
  (if (`Actor.ActorHasTag` OtherActor "Player")
    (bind _returnvalue (`KismetSystemLibrary.K2_SetTimerDelegate` (`|CreateDelegate` :!event `Refresh Widget`) 0.5 true))))

(event `self.Hide Widget`
  (params (OverlappedComponent :type "PrimitiveComponent Object Reference") (OtherActor :type "Actor Object Reference") (OtherComp :type "PrimitiveComponent Object Reference") (OtherBodyIndex :type Integer))
  (`parent.Hide Widget` OverlappedComponent OtherActor OtherComp OtherBodyIndex)
  (if (`Actor.ActorHasTag` OtherActor "Player")
    (`KismetSystemLibrary.K2_ClearAndInvalidateTimerHandle` (stale `self.Show Widget` _returnvalue))))

(fn `Get Interact Key`
  (returns (`Interact Key as Text` :type Text))
  (bind _returnvalue (`GameplayStatics.GetPlayerCharacter` 0))
  (bind _returnvalue_2 (`Actor.GetComponentByClass` _returnvalue "/Game/ActorComponents/AC_ToolInventoryAndAbilities.AC_ToolInventoryAndAbilities_C"))
  (bind (_bsuccess _held_object) (message `/Game/Interfaces/BPI_GetFromPlayer.Get Held Object` _returnvalue))
  (if _bsuccess
    (`KismetSystemLibrary.IsObjectOfSoftClass` _held_object "/Game/Objects/Pickup-able_Actors/BP_Pickup_Tin.BP_Pickup_Tin_C"
      (:`True`
        (return (`parent.Get Interact Key`)))
      (:`False`
        (return "")))
    (else
      (`/Engine/EditorBlueprintResources/StandardMacros.IsValid` _returnvalue_2
        (:`Is Valid`
          (if (== (`GameplayStatics.GetObjectClass` (`/Game/ActorComponents/AC_ToolInventoryAndAbilities.Current Tool` _returnvalue_2)) (`self.Tool`))
            (return (`KismetInputLibrary.Key_GetDisplayName` (`|GetArrayItem` (`EnhancedInputSubsystemInterface.QueryKeysMappedToAction` (pcsubsystem `EnhancedInputLocalPlayerSubsystem` (`GameplayStatics.GetPlayerController` 0)) "/Game/Characters/Player/Input/Actions/IA_UseAbility.IA_UseAbility")) false))
            (else
              _)))
        (:`Is Not Valid`
          _))
      (return ""))))

(fn `SetToolClass`
  (params (`Tool Class` :type "/Game/Tools/ToolActors/BP_ToolsBase Class Reference"))
  (set `self.Tool` `Tool Class`))