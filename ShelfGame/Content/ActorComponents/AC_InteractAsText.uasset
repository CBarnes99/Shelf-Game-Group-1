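; Actor component that shows an on-screen interact key prompt above its owner while a Player-tagged actor overlaps the owner's box collision.
; On BeginPlay it adds a screen-space widget component to the owner and binds the box's begin and end overlaps to show or clear a WBP_Interact widget.
; The key label comes from querying Enhanced Input for IA_Interact's current mapping, and RefreshWidget rebuilds the widget with that key.
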(event `self.ReceiveBeginPlay`
  (bind _returnvalue (`|AddComponentByClass` :`self` (`self.GetOwner`) :`Class` "/Script/UMG.WidgetComponent"))
  (bind _output_get (set `self.Interact Widget Component` _returnvalue))
  (`WidgetComponent.SetWidgetSpace` _output_get "Screen")
  (`WidgetComponent.SetDrawSize` _output_get (50.0 50.0))
  (`self.Get Collision Shape`))

(event `Get Collision Shape`
  (bind _returnvalue (`self.GetOwner`))
  (bind _returnvalue_2 (`Actor.GetComponentByClass` _returnvalue "/Script/Engine.BoxComponent"))
  (`/Engine/EditorBlueprintResources/StandardMacros.IsValid` _returnvalue_2
    (:`Is Valid`
      (add `PrimitiveComponent.OnComponentBeginOverlap` _returnvalue_2 (`|CreateDelegate` :!event `Show Widget`))
      (add `PrimitiveComponent.OnComponentEndOverlap` _returnvalue_2 (`|CreateDelegate` :!event `Hide Widget`)))
    (:`Is Not Valid`
      (`KismetSystemLibrary.PrintString` (`KismetTextLibrary.Conv_TextToString` (`|FormatText` "{owner} doesnt have a box collision" _returnvalue)) true true (struct :`R` 1.0 :`B` 0.077122 :`A` 1.0) 10.0))))

(event `Show Widget`
  (params (OverlappedComponent :type "PrimitiveComponent Object Reference") (OtherActor :type "Actor Object Reference") (OtherComp :type "PrimitiveComponent Object Reference") (OtherBodyIndex :type Integer) (bFromSweep :type Boolean) (SweepResult :type "HitResult Structure (by ref)"))
  (bind _interact_widget_component (`self.Interact Widget Component`))
  (if (`Actor.ActorHasTag` OtherActor "Player")
    (bind _returnvalue (`|CreateWidget` "/Game/Widgets/WBP_Interact.WBP_Interact_C" null (`self.Get Interact Key`)))
    (bind _output_get (set `self.Widget Reference` _returnvalue))
    (`WidgetComponent.SetWidget` _interact_widget_component _output_get)
    (`SceneComponent.K2_SetWorldLocation` _interact_widget_component (`self.Get Widget Display Location`) false false)
    (else
      (`KismetSystemLibrary.PrintString` "Actor Doesnt Have 'Player' Tag "))))

(event `Hide Widget`
  (params (OverlappedComponent :type "PrimitiveComponent Object Reference") (OtherActor :type "Actor Object Reference") (OtherComp :type "PrimitiveComponent Object Reference") (OtherBodyIndex :type Integer))
  (if (`Actor.ActorHasTag` OtherActor "Player")
    (set `self.Widget Reference` null)
    (`WidgetComponent.SetWidget` (`self.Interact Widget Component`) null)
    (else
      (`KismetSystemLibrary.PrintString` "Actor Doesnt Have 'Player' Tag "))))

(event `Refresh Widget`
  (bind _interact_widget_component (`self.Interact Widget Component`))
  (set `self.Widget Reference` null)
  (`WidgetComponent.SetWidget` (`self.Interact Widget Component`) null)
  (bind _returnvalue (`|CreateWidget` "/Game/Widgets/WBP_Interact.WBP_Interact_C" null (`self.Get Interact Key`)))
  (bind _output_get (set `self.Widget Reference` _returnvalue))
  (`WidgetComponent.SetWidget` _interact_widget_component _output_get)
  (`SceneComponent.K2_SetWorldLocation` _interact_widget_component (`self.Get Widget Display Location`) false false))

(fn `Get Interact Key`
  (returns (`Interact Key as Text` :type Text))
  (return (`KismetInputLibrary.Key_GetDisplayName` (`|GetArrayItem` (`EnhancedInputSubsystemInterface.QueryKeysMappedToAction` (pcsubsystem `EnhancedInputLocalPlayerSubsystem` (`GameplayStatics.GetPlayerController` 0)) "/Game/Characters/Player/Input/Actions/IA_Interact.IA_Interact")) false)))

(fn `Get Widget Display Location`
  (returns (`DIsplay Loc` :type "Vector Structure"))
  (return (+ (`Actor.K2_GetActorLocation` (`self.GetOwner`)) (0.0 0.0 20.0))))