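; Actor component that manages the player's collectible arms and the gameplay ability each one grants.
; On BeginPlay it adds an AbilitySystemComponent to its owner; gaining an arm stores it, equips it and gives its ability.
; Only the current arm stays visible, and input activates its ability by gameplay tag.
; A selection widget lists gained arms, suspending player input until one is chosen and equipped.
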(event `self.ReceiveBeginPlay`
  ; Give the owner an ability system component
  (bind _returnvalue (`|AddComponentByClass` (`self.GetOwner`) "/Script/GameplayAbilities.AbilitySystemComponent"))
  (set `self.Ability System` _returnvalue))

(event `Gain Arm`
  (params (Arm :type "Actor Object Reference") (Player :type "Character Object Reference") (`Socket Name` :type Name))
  (bind (_bsuccess _arm _ability_tag _ability) (message `/Game/Interfaces/BPI_Interact.PickupArm` Arm Player `Socket Name`))
  (`KismetSystemLibrary.PrintString` (`KismetTextLibrary.Conv_TextToString` (`|FormatText` "Is Pickup Arm Successful - {bool}" _bsuccess)) true true (struct :`G` 0.66 :`B` 1.0 :`A` 1.0) 3.0)
  (if _bsuccess
    (`KismetArrayLibrary.Array_AddUnique` (`self.Gained Tools`) _arm)
    (`self.SetCurrentArmAndAbility` _arm _ability_tag)
    (`AbilitySystemComponent.K2_GiveAbility` (`self.Ability System`) _ability 0 -1)))

(event `Display Inventory`
  (if (not (<= (`KismetArrayLibrary.Array_Length` (`self.Gained Tools`)) 0))
    (bind _returnvalue (`|CreateWidget` "/Game/Widgets/ToolSelection/WBP_ToolSelection.WBP_ToolSelection_C" null (`self.Gained Tools`)))
    (bind _output_get (set `self.Tool Selection` _returnvalue))
    (add `/Game/Widgets/ToolSelection/WBP_ToolSelection.Arm Selected` _output_get (`|CreateDelegate` :!event `Use New Arm Selected From Inventory`))
    (`UserWidget.AddToViewport` (`self.Tool Selection`) 0)
    (message `/Game/Interfaces/BPI_ToggleInputForDialogue.Toggle Input` (`GameplayStatics.GetPlayerController` 0) false false)))

(event `Use New Arm Selected From Inventory`
  (params (`Selected Arm` :type "/Game/Tools/ToolActors/BP_ToolsBase Object Reference") (`Ability Tag` :type "GameplayTagContainer Structure"))
  (bind _tool_selection (`self.Tool Selection`))
  (`self.SetCurrentArmAndAbility` `Selected Arm` `Ability Tag`)
  (`/Engine/EditorBlueprintResources/StandardMacros.IsValid` _tool_selection
    (:`Is Valid`
      (clear `/Game/Widgets/ToolSelection/WBP_ToolSelection.Arm Selected` _tool_selection)
      (`Widget.RemoveFromParent` _tool_selection)
      (set `self.Tool Selection` null))
    (:`Is Not Valid`
      (`KismetSystemLibrary.PrintString` "Arm Selection with AC_ArmInventoryAndAbilities Not Valid" true true (struct :`R` 1.0 :`G` 0.022888 :`A` 1.0) 10.0)))
  (message `/Game/Interfaces/BPI_ToggleInputForDialogue.Toggle Input` (`GameplayStatics.GetPlayerController` 0) true true))

(event `EnhancedInput|/Game/Characters/Player/Input/Actions/IA_UseAbility`
  (params (ActionValue :type Boolean) (ElapsedSeconds :type "Float (double-precision)") (TriggeredSeconds :type "Float (double-precision)") (InputAction :type "InputAction Object Reference" :default "/Game/Characters/Player/Input/Actions/IA_UseAbility.IA_UseAbility"))
  (bind _current_ability (`self.Current Ability`))
  ; Use the current ability that is equiped
  (:`Triggered`
    (bind _returnvalue (`AbilitySystemComponent.TryActivateAbilitiesByTag` (`self.Ability System`) _current_ability true))
    (`KismetSystemLibrary.PrintString` (`KismetTextLibrary.Conv_TextToString` (`|FormatText` "Ability - {ability}. Successfull - {successfull}" (`BlueprintGameplayTagLibrary.GetDebugStringFromGameplayTagContainer` _current_ability) _returnvalue)))))

(event `EnhancedInput|/Game/Characters/Player/Input/Actions/IA_DisplayArmInventory`
  (params (ActionValue :type Boolean) (ElapsedSeconds :type "Float (double-precision)") (TriggeredSeconds :type "Float (double-precision)") (InputAction :type "InputAction Object Reference" :default "/Game/Characters/Player/Input/Actions/IA_DisplayArmInventory.IA_DisplayArmInventory"))
  ; Display Arm Inventory
  (:`Triggered`
    (`self.Display Inventory`)))

(fn `SetCurrentArmAndAbility`
  (params (Arm :type "/Game/Tools/ToolActors/BP_ToolsBase Object Reference") (`Ability Tag` :type "GameplayTagContainer Structure"))
  (bind _current_tool (`self.Current Tool`))
  (`/Engine/EditorBlueprintResources/StandardMacros.IsValid` _current_tool
    (:`Is Valid`
      (`Actor.SetActorHiddenInGame` _current_tool true))
    (:`Is Not Valid`
      _))
  (`Actor.SetActorHiddenInGame` Arm false)
  (bind _output_get (set `self.Current Tool` Arm))
  (bind _output_get_2 (set `self.Current Ability` `Ability Tag`))
  (`KismetSystemLibrary.PrintString` (`KismetTextLibrary.Conv_TextToString` (`|FormatText` "New Arm - {arm} \nNew Ability - {ability}" _output_get (`BlueprintGameplayTagLibrary.GetDebugStringFromGameplayTagContainer` _output_get_2))) true true (struct :`G` 0.66 :`B` 1.0 :`A` 1.0) 10.0))