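; BP_Objective_GiveObject is a quest objective that tracks handing a set of objects to an NPC.
; GaveObjectToNPC increments a received count, then finishes the objective when it equals the ObjectToGive list length, or signals an objective update otherwise.
; It returns the finished state and the received-minus-required difference, which GiveObjectFinishedCheck passes through.
; Completion progress is the ratio of received to required objects.
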(fn `GaveObjectToNPC`
  (returns (`Objective Finished` :type Boolean) (`Amount Still Needed` :type Integer))
  (bind _amount_recieved (`self.Amount Recieved`))
  (bind _returnvalue (`KismetArrayLibrary.Array_Length` (`self.Object To Give`)))
  (bind _returnvalue_2 (== _returnvalue _amount_recieved))
  (`/Engine/EditorBlueprintResources/StandardMacros.IncrementInt` (`self.Amount Recieved`)
    (:`  `
      (if _returnvalue_2
        (`self.Finish Objective`)
        (else
          (`self.Update Objective` self)))
      (return _returnvalue_2 (- _amount_recieved _returnvalue)))))

(fn `Get Completion Progress`
  (returns (`Completion Rate` :type "Float (double-precision)"))
  (return (/ (`KismetMathLibrary.Conv_IntToDouble` (`self.Amount Recieved`)) (`KismetMathLibrary.Conv_IntToDouble` (`KismetArrayLibrary.Array_Length` (`self.Object To Give`))))))

(fn `Give Object Finished Check`
  (returns (`bObjective Finished` :type Boolean) (`Amount Still Needed` :type Integer))
  (bind (_objective_finished _amount_still_needed) (`self.GaveObjectToNPC`))
  (return _objective_finished _amount_still_needed))