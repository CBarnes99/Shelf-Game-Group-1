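; Composite quest objective that groups sub-objectives and finishes once all of them are completed.
; On activation it either starts every sub-objective at once or, with CompleteInOrder, chains them by activating the next inactive one as each finishes.
; It binds to child update and finish events to forward updates upward.
; Completion progress is the equally weighted average of the sub-objectives' progress.
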(event `self.Activate Objective`
  (`parent.Activate Objective`)
  (for _array_element (`self.Sub Objectives`)
    (add `self.Update Objective` _array_element (`|CreateDelegate` :!event `Foward Update Objective`)))
  (if (`self.Complete In Order`)
    (`self.Activate Next Objective In Order`)
    (else
      (`self.Activate All Objectives`)
      (`self.Update Objective` self))))

(event `Foward Update Objective` :!signature `self.Update Objective`
  (params (Objective :type "/Game/Quests/ObjectiveTypes/BP_BaseObjective Object Reference"))
  (`self.Update Objective` self))

(event `Objective Finished` :!signature `self.Finished Objective`
  (params (Objective :type "/Game/Quests/ObjectiveTypes/BP_BaseObjective Object Reference"))
  (`self.Check Objective Collection Finished`)
  (remove `self.Finished Objective` Objective (`|CreateDelegate` :!event `Objective Finished`))
  (`self.Update Objective` self))

(event `On Sequential Objective Finished` :!signature `self.Finished Objective`
  (params (Objective :type "/Game/Quests/ObjectiveTypes/BP_BaseObjective Object Reference"))
  (remove `self.Finished Objective` Objective (delegate `On Sequential Objective Finished`))
  (`self.Activate Next Objective In Order`)
  (`self.Update Objective` self))

(fn `Activate All Objectives`
  (for _array_element (`self.Sub Objectives`)
    (`self.Activate Objective` _array_element)
    (add `self.Finished Objective` _array_element (`|CreateDelegate` :!event `Objective Finished`))))

(fn `Activate Next Objective In Order`
  (for _array_element (`self.Sub Objectives`)
    (if (not (`/Game/Quests/ObjectiveTypes/BP_BaseObjective.bIsActive` _array_element))
      (`self.Activate Objective` _array_element)
      (add `self.Finished Objective` _array_element (`|CreateDelegate` :!event `On Sequential Objective Finished`))
      (return)))
  (`self.Check Objective Collection Finished`))

(fn `Check Objective Collection Finished`
  (for _array_element (`self.Sub Objectives`)
    (if (not (`/Game/Quests/ObjectiveTypes/BP_BaseObjective.bIsCompleted` _array_element))
      (return)))
  (`self.Finish Objective`))

(fn `Get Completion Progress`
  (returns (`Completion Rate` :type "Float (double-precision)"))
  (locals (`Complete Rate` :type "Float (double-precision)"))
  (for _array_element (`self.Sub Objectives`)
    (bind _completion_rate (`self.Get Completion Progress` _array_element))
    (set `local.Complete Rate` (+ (`local.Complete Rate`) (/ _completion_rate (`KismetMathLibrary.Conv_IntToDouble` (`KismetArrayLibrary.Array_Length` (`self.Sub Objectives`)))))))
  (return (`local.Complete Rate`)))