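; BP_BaseObjective is the base quest objective, tracking whether it is active and completed.
; Finishing runs only once: it sets the completed flag, prints a debug message with the objective's gameplay tag and calls FinishedObjective to notify the quest.
; Completed state can be exported as a tag list and reapplied from one through the same finish path, while progress reports as all-or-nothing.
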(fn `Activate Objective`
  ; Sets the objective active
  (set `self.bIsActive` true))

(fn `Finish Objective`
  ; Tells the quest that the objective is bound to that this quest is finished
  (if (not (`self.bIsCompleted`))
    (set `self.bIsCompleted` true)
    (`KismetSystemLibrary.PrintString` null (`KismetTextLibrary.Conv_TextToString` (`|FormatText` "{Objective ID} Has been Completed" (`BlueprintGameplayTagLibrary.GetDebugStringFromGameplayTag` (`self.ObjectiveID`)))) true true (struct :`R` 0.054123 :`G` 1.0 :`B` 0.223677 :`A` 1.0) 5.0)
    (`self.Finished Objective` self)))

(fn `Get Completed Objectives`
  (returns (`Completed Objectives` :type "Array of GameplayTag Structure"))
  (if (`self.bIsCompleted`)
    (return (`|MakeArray` (`self.ObjectiveID`)))
    (else
      (return))))

(fn `Get Completion Progress`
  (returns (`Completion Rate` :type "Float (double-precision)"))
  (return (`KismetMathLibrary.SelectFloat` 1.0 0.0 (`self.bIsCompleted`))))

(fn `Set Objective Complete By ID`
  (params (`Completed Objectives` :type "Array of GameplayTag Structure"))
  (if (`KismetArrayLibrary.Array_Contains` `Completed Objectives` (`self.ObjectiveID`))
    (`self.Finish Objective`)))