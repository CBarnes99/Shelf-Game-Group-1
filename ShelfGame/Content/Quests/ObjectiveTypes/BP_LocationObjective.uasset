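; BP_LocationObjective is a quest objective that completes when the player reaches a location.
; On activation it runs the parent objective logic and binds to the begin-overlap event of its LocationTrigger actor.
; An overlapping actor tagged Player finishes the objective only if it has an AC_QuestOrganiser component; otherwise an error message prints on screen.
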(fn `Activate Objective`
  (`parent.Activate Objective`)
  (add `Actor.OnActorBeginOverlap` (`self.Location Trigger`) (`|CreateDelegate` :!event `On Location Reached`)))

(fn `On Location Reached`
  (params (OverlappedActor :type "Actor Object Reference") (OtherActor :type "Actor Object Reference"))
  (if (`Actor.ActorHasTag` OtherActor "Player")
    (`/Engine/EditorBlueprintResources/StandardMacros.IsValid` (`Actor.GetComponentByClass` OtherActor "/Game/ActorComponents/AC_QuestOrganiser.AC_QuestOrganiser_C")
      (:`Is Valid`
        (`self.Finish Objective`))
      (:`Is Not Valid`
        (`KismetSystemLibrary.PrintString` null "Player Doenst Have AC_QuestOrganiser Attached" true true (struct :`R` 1.0 :`G` 0.033796 :`A` 1.0) 20.0)))))