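; Base quest Blueprint that child quests subclass, building an objective tree and reporting its progress and completion.
; BeginPlay stores the result of InitializeObjectives, a stub that prints a red error unless overridden, and takes QuestID from the root objective.
; StartQuest activates the root and binds to it and each sub-objective.
; Sub-objective updates or completions raise quest-updated calls, while only root completion raises quest completed.
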(event `self.ReceiveBeginPlay`
  (bind _objectives (`self.Initialize Objectives`))
  (bind _output_get (set `self.Objectives` _objectives))
  (set `self.QuestID` (`/Game/Quests/ObjectiveTypes/BP_Objective_Base.ObjectiveID` _output_get)))

(event `Start Quest`
  (bind _objectives (`self.Objectives`))
  (`/Game/Quests/ObjectiveTypes/BP_Objective_Base.Activate Objective` _objectives)
  (add `/Game/Quests/ObjectiveTypes/BP_Objective_Base.Finished Objective` _objectives (delegate `On Quest Completed`))
  (add `/Game/Quests/ObjectiveTypes/BP_Objective_Base.Update Objective` _objectives (delegate `On Quest Updated`))
  (for _array_element (`/Game/Quests/ObjectiveTypes/BP_Objective_Collection.Sub Objectives` (`self.Objectives`))
    (add `/Game/Quests/ObjectiveTypes/BP_Objective_Base.Update Objective` _array_element (delegate `On Updated Objective`))
    (add `/Game/Quests/ObjectiveTypes/BP_Objective_Base.Finished Objective` _array_element (delegate `On Updated Objective`)))
  (`self.Quest Updated`))

(event `On Updated Objective`
  (params (Objective :type "/Game/Quests/ObjectiveTypes/BP_Objective_Base Object Reference"))
  (`self.Quest Updated`))

(event `On Quest Completed`
  (params (Objective :type "/Game/Quests/ObjectiveTypes/BP_Objective_Base Object Reference"))
  (`self.Completed Quest` self))

(event `On Quest Updated`
  (params (Objective :type "/Game/Quests/ObjectiveTypes/BP_Objective_Base Object Reference"))
  (`self.Quest Updated`))

(fn `Initialize Objectives`
  (returns (Objectives :type "/Game/Quests/ObjectiveTypes/BP_Objective_Collection Object Reference"))
  (`KismetSystemLibrary.PrintString` "PARENT BASE QUEST INITALIZE CALLED! OVERRIDE THIS FUNCTION IN CHILD CLASS!" true true (struct :`R` 1.0 :`G` 0.018695 :`A` 1.0) 100.0)
  (return null))

(fn `UserConstructionScript`)