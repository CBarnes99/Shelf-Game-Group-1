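; BP_TestQuest is a test quest that asks the player to move to three locations in sequence.
; Its Initialize Objectives function constructs three location objectives, each tied to its own trigger, on-screen name and hierarchical objective ID.
; It wraps them in an ordered objective collection and returns that as the quest's root objective.
; The event graph and construction script add no logic of their own.
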(fn `Initialize Objectives`
  (returns (Objectives :type "/Game/Quests/ObjectiveTypes/BP_ObjectiveCollection Object Reference"))
  (bind _returnvalue (`|GenericCreateObject` "/Game/Quests/ObjectiveTypes/BP_LocationObjective.BP_LocationObjective_C" (`self.Location Test 1`) "Location test 1" (struct :`TagName` "Quests.Test.loc1")))
  (bind _returnvalue_2 (`|GenericCreateObject` "/Game/Quests/ObjectiveTypes/BP_LocationObjective.BP_LocationObjective_C" (`self.Location Test 2`) "Location test 2" (struct :`TagName` "Quests.Test.loc2")))
  (bind _returnvalue_3 (`|GenericCreateObject` "/Game/Quests/ObjectiveTypes/BP_LocationObjective.BP_LocationObjective_C" (`self.Location Test 3`) "Location test 3" (struct :`TagName` "Quests.Test.loc3")))
  (bind _returnvalue_4 (`|GenericCreateObject` "/Game/Quests/ObjectiveTypes/BP_ObjectiveCollection.BP_ObjectiveCollection_C" (`|MakeArray` _returnvalue _returnvalue_2 _returnvalue_3 :!type "/Game/Quests/ObjectiveTypes/BP_BaseObjective Object Reference") true "Move to locations!" (struct :`TagName` "Quests.Test")))
  (return _returnvalue_4))

(fn `UserConstructionScript`
  (`parent.UserConstructionScript`))