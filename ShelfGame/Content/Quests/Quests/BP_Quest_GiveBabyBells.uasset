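; Quest Blueprint for helping Piccolina by finding her bells.
; InitializeObjectives builds a "Help Piccolina" collection objective wrapping a give-actors objective that uses ObjectToGive and shows a progress bar.
; On BeginPlay it binds to quest completion, which enables the assigned line climb, or prints an on-screen error if none is set.
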(event `self.ReceiveBeginPlay`
  (`parent.ReceiveBeginPlay`)
  (add `self.Quest Completed` self (delegate `Set LineClimb Enabled`)))

(event `Set LineClimb Enabled` :!signature `self.Quest Completed`
  (params (`Completed Quest` :type "/Game/Quests/Quests/BP_BaseQuest Object Reference"))
  (bind _lineclimb_to_enable_on_quest_finished (`self.LineClimb To Enable On Quest Finished`))
  (`/Engine/EditorBlueprintResources/StandardMacros.IsValid` _lineclimb_to_enable_on_quest_finished
    (:`Is Valid`
      (set `/Game/Objects/BP_LineClimb.bIsEnabled` true _lineclimb_to_enable_on_quest_finished))
    (:`Is Not Valid`
      (`KismetSystemLibrary.PrintString` (`KismetTextLibrary.Conv_TextToString` (`|FormatText` self "Line Climb Not Set Within {self} ")) true true (struct :`R` 1.0 :`G` 0.006029 :`A` 1.0) 10.0))))

(fn `Initialize Objectives`
  (returns (Objectives :type "/Game/Quests/ObjectiveTypes/BP_Objective_Collection Object Reference"))
  (bind _returnvalue (`|GenericCreateObject` "/Game/Quests/ObjectiveTypes/BP_Objective_GiveActors.BP_Objective_GiveActors_C" (`self.Object To Give`) "Find Piccolina's Bells" (struct :`TagName` "Quests.Piccolina.Bells") true))
  (bind _returnvalue_2 (`|GenericCreateObject` "/Game/Quests/ObjectiveTypes/BP_Objective_Collection.BP_Objective_Collection_C" (`|MakeArray` _returnvalue :!type "/Game/Quests/ObjectiveTypes/BP_Objective_Base Object Reference") false "Help Piccolina" (struct :`TagName` "Quests.Piccolina")))
  (return _returnvalue_2))

(fn `UserConstructionScript`
  (`parent.UserConstructionScript`))