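; Base actor for pickup tools that attach to the player who interacts with them.
; Interact snaps the tool to a configurable socket on the player's mesh, allows only one pickup, and disables the Cube's collision.
; It then registers the tool through GainTool on the player's AC_ToolInventoryAndAbilities component.
; Failures print a message and return false, though a missing component still leaves the tool attached.
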(fn `Interact`
  (params (Interactor :type "Character Object Reference"))
  (returns (bSuccess :type Boolean))
  (locals (Player :type "Character Object Reference"))
  (bind _returnvalue (`self.GetComponentByClass` (`local.Player`) "/Game/ActorComponents/AC_ToolInventoryAndAbilities.AC_ToolInventoryAndAbilities_C"))
  (bind _output_get (set `local.Player` Interactor))
  (if (and (not (`self.Has Been Picked Up`)) (`KismetSystemLibrary.IsValid` _output_get))
    (bind _returnvalue_2 (`self.K2_AttachToComponent` (`Character.Mesh` _output_get) (`self.Socket To Attach To`) "SnapToTarget" "SnapToTarget" "SnapToTarget"))
    (bind _output_get_2 (set `self.Has Been Picked Up` _returnvalue_2))
    (if _output_get_2
      (`PrimitiveComponent.SetCollisionEnabled` (`self.Cube`) "NoCollision")
      (`/Engine/EditorBlueprintResources/StandardMacros.IsValid` _returnvalue
        (:`Is Valid`
          (`/Game/ActorComponents/AC_ToolInventoryAndAbilities.Gain Tool` _returnvalue self)
          (return (`self.Has Been Picked Up`)))
        (:`Is Not Valid`
          (`KismetSystemLibrary.PrintString` "Player Doesn't Have Tool Ability Component" true true (struct :`R` 1.0 :`B` 0.054096 :`A` 1.0) 10.0)
          (return false)))
      (else
        (`KismetSystemLibrary.PrintString` "Tool Failed To Attach To Mesh" true true (struct :`R` 1.0 :`G` 0.038732 :`A` 1.0) 10.0)
        (return false)))
    (else
      (`KismetSystemLibrary.PrintString` "Either Has Already Been Picked Up or Interactor Not Valid" true true (struct :`R` 1.0 :`G` 0.058149 :`A` 1.0) 10.0)
      (return false))))

(fn `UserConstructionScript`)