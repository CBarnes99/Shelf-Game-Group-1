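; BP_PlaneManager is a one-shot setup actor that shares position data among a set of plane actors.
; Its SetPlaneInformation event collects the world location of each plane's Cube component into PlaneYLocations.
; A second pass hands every plane that full list along with its own one-based index, then the manager destroys itself.
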(event `SetPlaneInformation`
  (for _array_element (`self.Planes`)
    (`KismetArrayLibrary.Array_Add` (`self.Plane Y Locations`) (`SceneComponent.K2_GetComponentLocation` (`/Game/Planes/BP_Planes.Cube` _array_element))))
  (for (_array_element_2 _array_index) (`self.Planes`)
    (`/Game/Planes/BP_Planes.Set Plane Information` _array_element_2 (`self.Plane Y Locations`) (+ _array_index 1)))
  (`self.K2_DestroyActor`))

(fn `UserConstructionScript`)