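; BP_Planes is a setup actor for one depth plane along Y, initialized with every plane's Y location and its own index.
; It scans actors overlapping its box, passing plane index, count and locations to any AC_PivotBetweenPlanes component.
; Actors with an unaligned AC_PlaneAlignedObject are snapped to the plane's Y, keeping X and Z, and notified.
; It then destroys itself, so it only serves as a one-shot initializer.
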(fn `Set Object Plane Pivots`
  (locals (`New Loc` :type "Vector Structure" :default (0.0 0.0 0.0)) (`Old Loc` :type "Vector Structure" :default (0.0 0.0 0.0)))
  (bind (_returnvalue_x _returnvalue_y) (`KismetMathLibrary.BreakVector` (`self.K2_GetActorLocation`)))
  (for _array_element (`PrimitiveComponent.GetOverlappingActors` (`self.Box`) "/Script/Engine.Actor")
    (bind _returnvalue (`self.GetComponentByClass` _array_element "/Game/ActorComponents/AC_PivotBetweenPlanes.AC_PivotBetweenPlanes_C"))
    (`/Engine/EditorBlueprintResources/StandardMacros.IsValid` _returnvalue
      (:`Is Valid`
        (`/Game/ActorComponents/AC_PivotBetweenPlanes.Set Plane Information` _returnvalue (`self.This Plane Index`) (`KismetArrayLibrary.Array_Length` (`self.Plane Y Locations`)) (`self.Plane Y Locations`)))
      (:`Is Not Valid`
        _))
    (bind _returnvalue_2 (`self.GetComponentByClass` _array_element "/Game/ActorComponents/AC_PlaneAlignedObject.AC_PlaneAlignedObject_C"))
    (`/Engine/EditorBlueprintResources/StandardMacros.IsValid` _returnvalue_2
      (:`Is Valid`
        (if (not (`/Game/ActorComponents/AC_PlaneAlignedObject.bIsAligned` _returnvalue_2))
          (bind (_returnvalue_x_2 _returnvalue_y_2 _returnvalue_z) (`KismetMathLibrary.BreakVector` (`self.K2_GetActorLocation` _array_element)))
          (bind _returnvalue_3 (`KismetMathLibrary.MakeVector` _returnvalue_x_2 _returnvalue_y _returnvalue_z))
          (`self.K2_SetActorLocation` _array_element _returnvalue_3 false false)
          (`/Game/ActorComponents/AC_PlaneAlignedObject.Aligned` _returnvalue_2 _returnvalue_3)))))
  (`self.K2_DestroyActor`))

(fn `Set Plane Information`
  (params (`Plane Locs` :type "Array of Vector Structure") (Index :type Integer))
  (set `self.Plane Y Locations` `Plane Locs`)
  (set `self.This Plane Index` Index)
  (`self.Set Object Plane Pivots`))

(fn `UserConstructionScript`)