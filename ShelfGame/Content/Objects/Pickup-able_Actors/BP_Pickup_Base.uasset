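; Base Blueprint for pickup-able objects that show an interact key prompt based on the player's current tool.
; Once its plane-alignment component reports aligned, the mesh teleports to the aligned start location and simulates physics constrained to the XZ plane.
; The prompt shows the use-ability key only with the pickup tool equipped and empty hands.
; Tool-equip events refresh it while the player overlaps the box, and bindings clear on destruction.
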(event `self.ReceiveBeginPlay`
  (bind _returnvalue (`self.GetComponentByClass` (`GameplayStatics.GetPlayerCharacter` 0) "/Game/ActorComponents/AC_ToolInventoryAndAbilities.AC_ToolInventoryAndAbilities_C"))
  (add `/Game/ActorComponents/AC_PlaneAlignedObject.AlignedEvent` (`self.AC_PlaneAlignedObject`) (delegate `Enable Simulate Physics`))
  ; Binds to update the interact text and unbind them when the pickup actor is destoryed
  (add `/Game/ActorComponents/AC_InteractAsText.Set Interact Key Event` (`self.AC_InteractAsText`) (delegate `Set Interact Text`))
  (`/Engine/EditorBlueprintResources/StandardMacros.IsValid` _returnvalue
    (:`Is Valid`
      (add `/Game/ActorComponents/AC_ToolInventoryAndAbilities.Tool Equipped` _returnvalue (delegate `Update Interact Text`))
      (add `self.OnDestroyed` (delegate `Unbind Events`)))))

(event `Set Interact Text`
  (bind (_input_action _index) (`self.Get Interact Text `))
  ; Binds to update the interact text and unbind them when the pickup actor is destoryed
  (`/Game/ActorComponents/AC_InteractAsText.Set Interact Key` (`self.AC_InteractAsText`) _input_action _index))

(event `Update Interact Text`
  ; Binds to update the interact text and unbind them when the pickup actor is destoryed
  (if (`self.Player In Range`)
    (`/Game/ActorComponents/AC_InteractAsText.Refresh Widget` (`self.AC_InteractAsText`))))

(event `Unbind Events` :!signature `self.OnDestroyed`
  (params (DestroyedActor :type "Actor Object Reference"))
  ; Binds to update the interact text and unbind them when the pickup actor is destoryed
  (remove `/Game/ActorComponents/AC_InteractAsText.Set Interact Key Event` (`self.AC_InteractAsText`) (delegate `Set Interact Text`))
  (remove `/Game/ActorComponents/AC_ToolInventoryAndAbilities.Tool Equipped` (`self.GetComponentByClass` (`GameplayStatics.GetPlayerCharacter` 0) "/Game/ActorComponents/AC_ToolInventoryAndAbilities.AC_ToolInventoryAndAbilities_C") (delegate `Update Interact Text`)))

(event `Enable Simulate Physics`
  (bind _mesh (`self.Mesh`))
  ; When object has been aligned, enable physics
  (`SceneComponent.K2_SetWorldLocation` _mesh (`/Game/ActorComponents/AC_PlaneAlignedObject.Starting Loc` (`self.AC_PlaneAlignedObject`)) false true)
  (`PrimitiveComponent.SetConstraintMode` _mesh "XZPlane")
  (`PrimitiveComponent.SetSimulatePhysics` _mesh true))

(event `self.Box.OnComponentBeginOverlap`
  (params (OverlappedComponent :type "PrimitiveComponent Object Reference") (OtherActor :type "Actor Object Reference") (OtherComp :type "PrimitiveComponent Object Reference") (OtherBodyIndex :type Integer) (bFromSweep :type Boolean) (SweepResult :type "HitResult Structure (by ref)"))
  ; When player in range, set the bool check
  (if (`self.ActorHasTag` OtherActor "Player")
    (set `self.Player In Range` true)))

(event `self.Box.OnComponentEndOverlap`
  (params (OverlappedComponent :type "PrimitiveComponent Object Reference") (OtherActor :type "Actor Object Reference") (OtherComp :type "PrimitiveComponent Object Reference") (OtherBodyIndex :type Integer))
  ; When player in range, set the bool check
  (if (`self.ActorHasTag` OtherActor "Player")
    (set `self.Player In Range` false)))

(fn `Get Interact Text `
  (returns (`Input Action` :type "InputAction Object Reference") (Index :type Integer))
  (bind _returnvalue (`GameplayStatics.GetPlayerCharacter` 0))
  ; Gets the interact key based on the tool and the object the player is using
  (bind _current_tool (message `/Game/Interfaces/BPI_GetFromPlayer.Get Current Tool Class` _returnvalue))
  (bind _bsuccess (message `/Game/Interfaces/BPI_GetFromPlayer.Get Held Object` _returnvalue))
  (if (and (not _bsuccess) (== _current_tool "/Game/Tools/ToolActors/BP_Tools_Pickup.BP_Tools_Pickup_C"))
    (return "/Game/Characters/Player/Input/Actions/IA_UseAbility.IA_UseAbility" 0)
    (else
      (return null 0))))

(fn `UserConstructionScript`)