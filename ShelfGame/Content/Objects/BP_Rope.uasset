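; BP_Rope is a rope barrier that blocks the player until the Scissors ability cuts it.
; Construction and BeginPlay size the cable, cut halves, caps and collision from the rope's endpoint.
; Side triggers shift a blocking cube beyond the opposite side from the player, and the interact prompt's key follows the equipped tool.
; Cutting swaps the full cable for two dangling halves, unbinds events and destroys the blocking components after a short delay.
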(event OnComponentBeginOverlap(LeftCollision)
  (params (OverlappedComponent :type Primitive%20Component%20Object%20Reference) (OtherActor :type Actor%20Object%20Reference) (OtherComp :type Primitive%20Component%20Object%20Reference) (OtherBodyIndex :type Integer) (bFromSweep :type Boolean) (SweepResult :type Hit%20Result%20Structure%20%28by%20ref%29))
  ;[0.15 0.15 0.15 0.5] Sets the box collision position and sets if the player is in range
  (Utilities|OverlapCollisionCheck OverlappedComponent OtherActor
    (:Valid
      (Variables|/Script/Engine.PrimitiveComponent|SetbGenerateOverlapEvents (Variables|Default|GetRight%20Collision) false)
      (CallFunction|MoveBlockingCube true)
      (CallFunction|SetPlayerinRange))))

(event OnComponentEndOverlap(LeftCollision)
  (params (OverlappedComponent :type Primitive%20Component%20Object%20Reference) (OtherActor :type Actor%20Object%20Reference) (OtherComp :type Primitive%20Component%20Object%20Reference) (OtherBodyIndex :type Integer))
  ;[0.15 0.15 0.15 0.5] Sets the box collision position and sets if the player is in range
  (Utilities|OverlapCollisionCheck OverlappedComponent OtherActor
    (:Valid
      (Variables|/Script/Engine.PrimitiveComponent|SetbGenerateOverlapEvents (Variables|Default|GetRight%20Collision) true)
      (CallFunction|ResetBlockLocation)
      (CallFunction|SetPlayerNotinRange))))

(event OnComponentBeginOverlap(RightCollision)
  (params (OverlappedComponent :type Primitive%20Component%20Object%20Reference) (OtherActor :type Actor%20Object%20Reference) (OtherComp :type Primitive%20Component%20Object%20Reference) (OtherBodyIndex :type Integer) (bFromSweep :type Boolean) (SweepResult :type Hit%20Result%20Structure%20%28by%20ref%29))
  ;[0.15 0.15 0.15 0.5] Sets the box collision position and sets if the player is in range
  (Utilities|OverlapCollisionCheck OverlappedComponent OtherActor
    (:Valid
      (Variables|/Script/Engine.PrimitiveComponent|SetbGenerateOverlapEvents (Variables|Default|GetLeft%20Collision) false)
      (CallFunction|MoveBlockingCube false)
      (CallFunction|SetPlayerinRange))))

(event OnComponentEndOverlap(RightCollision)
  (params (OverlappedComponent :type Primitive%20Component%20Object%20Reference) (OtherActor :type Actor%20Object%20Reference) (OtherComp :type Primitive%20Component%20Object%20Reference) (OtherBodyIndex :type Integer))
  ;[0.15 0.15 0.15 0.5] Sets the box collision position and sets if the player is in range
  (Utilities|OverlapCollisionCheck OverlappedComponent OtherActor
    (:Valid
      (Variables|/Script/Engine.PrimitiveComponent|SetbGenerateOverlapEvents (Variables|Default|GetLeft%20Collision) true)
      (CallFunction|ResetBlockLocation)
      (CallFunction|SetPlayerNotinRange))))

(event Custom|Reset%20Block%20Location
  (bind _block_movement_cube (Variables|Default|GetBlock%20Movement%20Cube))
  ;[0.15 0.15 0.15 0.5] Resets the block to its starting loc
  (Utilities|IsValid _block_movement_cube
    (:Is%20Valid
      (Transformation|SetRelativeLocation _block_movement_cube (Variables|Default|GetBlock%20Starting%20Loc) false false)
      (Collision|SetCollisionEnabled _block_movement_cube "QueryOnly"))))

(event Custom|Move%20Blocking%20Cube
  (params (LeftCollisionInteracted :type Boolean))
  (bind _left_collision (Variables|Default|GetLeft%20Collision))
  (bind _right_collision (Variables|Default|GetRight%20Collision))
  (bind _returnvalue (select LeftCollisionInteracted _right_collision _left_collision))
  (bind _relativelocation (Variables|/Script/Engine.SceneComponent|GetRelativeLocation _returnvalue))
  ;[0.15 0.15 0.15 0.5] Moves the blocking cube location
  (Transformation|SetRelativeLocation (Variables|Default|GetBlock%20Movement%20Cube) (Math|Vector|MakeVector (.x _relativelocation) (* (.y _relativelocation) 2.0) (.z _relativelocation)) false false)
  (Collision|SetCollisionEnabled (Variables|Default|GetBlock%20Movement%20Cube) "QueryAndPhysics"))

(event Custom|Set%20Interact%20Key
  (bind (_input_action _index) (CallFunction|GetInteractKey))
  ;[0.15 0.15 0.15 0.5] Binds events for the text interact key
  (Default|SetInteractKey (Variables|Default|GetAC_InteractAsText) _input_action _index))

(event Custom|Update%20Interact%20Key
  ;[0.15 0.15 0.15 0.5] Binds events for the text interact key
  (if (Variables|Default|GetbPlayerInRange)
    (Default|RefreshWidget (Variables|Default|GetAC_InteractAsText))))

(event Custom|Set%20Player%20Not%20In%20Range
  ;[0.15 0.15 0.15 0.5] Set if player is in range for interaction
  (Variables|Default|SetbPlayerInRange false))

(event Custom|Set%20Player%20In%20Range
  ;[0.15 0.15 0.15 0.5] Set if player is in range for interaction
  (Variables|Default|SetbPlayerInRange true))

(event EventBeginPlay
  (bind _returnvalue (Game|GetPlayerCharacter 0))
  (bind _returnvalue_2 (Actor|GetComponentbyClass _returnvalue "/Game/ActorComponents/AC_ToolInventoryAndAbilities.AC_ToolInventoryAndAbilities_C"))
  ;[0.15 0.15 0.15 0.5] Sets the rope defaults at start
  (CallFunction|SetUpRope)
  (Variables|Default|SetBlock%20Starting%20Loc (Variables|/Script/Engine.SceneComponent|GetRelativeLocation (Variables|Default|GetBlock%20Movement%20Cube)))
  (CallFunction|ResetBlockLocation)
  ;[0.15 0.15 0.15 0.5] Binds events for the text interact key
  (EventDispatchers|BindEventtoSetInteractKeyEvent (Variables|Default|GetAC_InteractAsText) (delegate Custom|Set%20Interact%20Key))
  (Utilities|IsValid _returnvalue_2
    (:Is%20Valid
      (EventDispatchers|BindEventtoToolEquipped _returnvalue_2 (delegate Custom|Update%20Interact%20Key)))))

(fn ConstructionScript
  (CallFunction|SetUpRope))

(fn SetBeenCut
  (bind _leftcut (Variables|Default|GetLeftCut))
  (bind _rightcut (Variables|Default|GetRightCut))
  (bind _left_collision (Variables|Default|GetLeft%20Collision))
  (bind _fullrope (Variables|Default|GetFullRope))
  (bind _right_collision (Variables|Default|GetRight%20Collision))
  (bind _block_movement_cube (Variables|Default|GetBlock%20Movement%20Cube))
  ;[0.15 0.15 0.15 0.5] If the rope has been cut, disable the main rope and have the side ropes dangle
  (Variables|Default|SetbHasBeenCut true)
  (Rendering|SetVisibility _leftcut true false)
  (Collision|SetCollisionEnabled _leftcut "QueryAndPhysics")
  (Variables|/Script/CableComponent.CableComponent|SetbAttachEnd _leftcut false)
  (Rendering|SetVisibility _rightcut true false)
  (Collision|SetCollisionEnabled _rightcut "QueryAndPhysics")
  (Variables|/Script/CableComponent.CableComponent|SetbAttachEnd _rightcut false)
  (Collision|SetCollisionEnabled _fullrope "NoCollision")
  (Rendering|SetVisibility _fullrope false false)
  (Rendering|SetVisibility _block_movement_cube false false)
  (Collision|SetCollisionEnabled _block_movement_cube "NoCollision")
  (Collision|SetCollisionEnabled _left_collision "NoCollision")
  (Variables|/Script/Engine.PrimitiveComponent|SetbGenerateOverlapEvents _left_collision false)
  (Variables|/Script/Engine.PrimitiveComponent|SetbGenerateOverlapEvents _right_collision false)
  (Collision|SetCollisionEnabled _right_collision "NoCollision")
  (EventDispatchers|UnbindEventfromToolEquipped (Actor|GetComponentbyClass (Game|GetPlayerCharacter 0) "/Game/ActorComponents/AC_ToolInventoryAndAbilities.AC_ToolInventoryAndAbilities_C") (EventDispatchers|CreateEvent :!event Custom|Update%20Interact%20Key))
  (EventDispatchers|UnbindEventfromSetInteractKeyEvent (Variables|Default|GetAC_InteractAsText) (EventDispatchers|CreateEvent :!event Custom|Set%20Interact%20Key))
  (Utilities|Time|SetTimerbyFunctionName 0 "Destroy Components" 0.1))

(fn SetUpRope
  (bind _left_cap (Variables|Default|GetLeft%20Cap))
  (bind _right_cap (Variables|Default|GetRight%20Cap))
  (bind _right_collision (Variables|Default|GetRight%20Collision))
  (bind _block_movement_cube (Variables|Default|GetBlock%20Movement%20Cube))
  (bind _fullrope (Variables|Default|GetFullRope))
  (bind _fullrope_2 (Variables|Default|GetFullRope))
  (bind _left_collision (Variables|Default|GetLeft%20Collision))
  (bind _leftcut (Variables|Default|GetLeftCut))
  (bind _rightcut (Variables|Default|GetRightCut))
  ;[0.15 0.15 0.15 0.5] Setup the two cut halfs
  (Variables|/Script/CableComponent.CableComponent|SetCableWidth _fullrope_2 (Math|Float|Clamp(Float) (Variables|Default|GetRope%20Width) 1.0 5e+01))
  (Variables|/Script/CableComponent.CableComponent|SetCableLength _fullrope_2 (/ (Math|Vector|Distance(Vector) (Variables|/Script/CableComponent.CableComponent|GetEndLocation _fullrope_2) "0, 0, 0") 1.3))
  (Rendering|Material|SetMaterial (Variables|Default|GetFullRope) 0 (Variables|Default|GetRope%20Material))
  (Variables|/Script/CableComponent.CableComponent|SetCableLength _leftcut (/ (Variables|/Script/CableComponent.CableComponent|GetCableLength _fullrope_2) 2.0))
  (Variables|/Script/CableComponent.CableComponent|SetEndLocation _leftcut (/ (Variables|/Script/CableComponent.CableComponent|GetEndLocation _fullrope_2) 2.0))
  (Variables|/Script/CableComponent.CableComponent|SetCableWidth _leftcut (Variables|/Script/CableComponent.CableComponent|GetCableWidth _fullrope_2))
  (Rendering|Material|SetMaterial _leftcut 0 (Variables|Default|GetRope%20Material))
  (Transformation|SetRelativeLocation _rightcut (Variables|/Script/CableComponent.CableComponent|GetEndLocation _fullrope_2) false false)
  (Variables|/Script/CableComponent.CableComponent|SetCableLength _rightcut (/ (Variables|/Script/CableComponent.CableComponent|GetCableLength _fullrope_2) 2.0))
  (Variables|/Script/CableComponent.CableComponent|SetEndLocation _rightcut (/ (Variables|/Script/CableComponent.CableComponent|GetEndLocation _fullrope_2) 2.0))
  (Variables|/Script/CableComponent.CableComponent|SetCableWidth _rightcut (Variables|/Script/CableComponent.CableComponent|GetCableWidth _fullrope_2))
  (Rendering|Material|SetMaterial _rightcut 0 (Variables|Default|GetRope%20Material))
  (Rendering|SetVisibility (Variables|Default|GetLeftCut) false false)
  (Rendering|SetVisibility (Variables|Default|GetRightCut) false false)
  ;[0.15 0.15 0.15 0.5] Set Midpoint for Collisions
  (bind _output_get (LocalVariables|SetMidpoint (|(((b-a)/2)+a) (Variables|/Script/CableComponent.CableComponent|GetEndLocation (Variables|Default|GetFullRope)) (Variables|/Script/Engine.SceneComponent|GetRelativeLocation _left_collision))))
  (Transformation|SetRelativeLocation _left_collision (Math|Vector|MakeVector (.x _output_get) (Variables|Default|GetCollision%20Y%20Loc) (.z _output_get)) false false)
  (Components|Box|SetBoxExtent _left_collision (Math|Vector|MakeVector (/ (Variables|/Script/CableComponent.CableComponent|GetCableLength (Variables|Default|GetFullRope)) 2.0) 3e+01 1e+01) true)
  (Transformation|SetRelativeLocation _right_collision (Math|Vector|MakeVector (.x (LocalVariables|GetMidpoint)) (* (Variables|Default|GetCollision%20Y%20Loc) -1.0) (.z (LocalVariables|GetMidpoint))) false false)
  (Components|Box|SetBoxExtent _right_collision (Math|Vector|MakeVector (/ (Variables|/Script/CableComponent.CableComponent|GetCableLength (Variables|Default|GetFullRope)) 2.0) 3e+01 1e+01) true)
  ;[0.15 0.15 0.15 0.5] Set Block Movement Cube Location
  (Transformation|SetRelativeLocation _block_movement_cube (- (LocalVariables|GetMidpoint) "0.000000,10.000000,0.000000") false false)
  (Transformation|SetRelativeScale3D _block_movement_cube (Math|Vector|MakeVector (/ (Variables|/Script/CableComponent.CableComponent|GetCableLength (Variables|Default|GetFullRope)) 8e+01) 0.1 3.0))
  ;[0.15 0.15 0.15 0.5] Setup Rope Caps
  (Transformation|SetRelativeLocation _left_cap (Variables|/Script/Engine.SceneComponent|GetRelativeLocation _fullrope) false false)
  (Rendering|Material|SetMaterial _left_cap 0 (Variables|Default|GetRope%20Material))
  (Transformation|SetRelativeScale3D _left_cap (Math|Conversions|ToVector(Float) (/ (Variables|/Script/CableComponent.CableComponent|GetCableWidth _fullrope) 1e+02)))
  (Transformation|SetRelativeLocation _right_cap (Variables|/Script/CableComponent.CableComponent|GetEndLocation _fullrope) false false)
  (Rendering|Material|SetMaterial _right_cap 0 (Variables|Default|GetRope%20Material))
  (Transformation|SetRelativeScale3D _right_cap (Math|Conversions|ToVector(Float) (/ (Variables|/Script/CableComponent.CableComponent|GetCableWidth _fullrope) 1e+02))))

(fn DestroyComponents
  ;[0.15 0.15 0.15 0.5] Destroys unessacary components after being cut
  (Components|DestroyComponent (Variables|Default|GetLeft%20Collision))
  (Components|DestroyComponent (Variables|Default|GetRight%20Collision))
  (Components|DestroyComponent (Variables|Default|GetBlock%20Movement%20Cube))
  (Components|DestroyComponent (Variables|Default|GetFullRope)))

(fn GetInteractKey
  (bind _returnvalue (Game|GetPlayerCharacter 0))
  (bind _returnvalue_2 (Actor|GetComponentbyClass _returnvalue "/Game/ActorComponents/AC_ToolInventoryAndAbilities.AC_ToolInventoryAndAbilities_C"))
  ;[0.15 0.15 0.15 0.5] Gets the interact Key
  (Utilities|IsValid _returnvalue_2
    (:Is%20Valid
      (if (== (Utilities|GetClass (Variables|/Game/ActorComponents/AC_ToolInventoryAndAbilities.AC_ToolInventoryAndAbilities_C|GetCurrent%20Tool _returnvalue_2)) "/Game/Tools/ToolActors/BP_Tools_Scissors.BP_Tools_Scissors_C")
        (return "/Game/Characters/Player/Input/Actions/IA_UseAbility.IA_UseAbility" 0)
        (else
          (return 0 0))))))

(fn CutRope
  (params (Interactor :type Character%20Object%20Reference))
  ;[0.15 0.15 0.15 0.5] Called from Scissors Ability to cut the rope
  (if (not (Variables|Default|GetbHasBeenCut))
    (Utilities|IsValid Interactor
      (:Is%20Valid
        (CallFunction|SetBeenCut)
        (return true))
      (:Is%20Not%20Valid
        (Development|PrintString "Interactor Not Valid On Rope" true true "(R=1.000000,G=0.076353,B=0.000000,A=1.000000)")
        (return false)))
    (else
      (Development|PrintString "Rope Has Already Been Cut" true true "(R=1.000000,G=0.076353,B=0.000000,A=1.000000)")
      (return false))))