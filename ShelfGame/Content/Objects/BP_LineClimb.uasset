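; BP_LineClimb is an interactable climbable that carries the player between the top and bottom of a ladder.
; Interact checks whether the interactor overlaps TopCol or BaseCol, snaps it to that end and plays the matching timeline.
; The timelines lerp the player cached at BeginPlay to the opposite end, finishing slightly above LadderTop when ascending.
; On finish, the player's starting Y is restored and HasInteracted clears to allow reuse.
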(event `self.ReceiveBeginPlay`
  (bind _asbp_player (cast `/Game/Characters/Player/BP_Player` (`GameplayStatics.GetPlayerCharacter` 0)))
  (set `self.BpPlayer` _asbp_player))

(event `TimeLineStart`
  (bind (_direction _newtrack_0) (`Timeline|Climb` :!via `PlayFromStart`)
    (:`Update`
      (bind _output_get (set `self.EndActorLocation` (`SceneComponent.K2_GetComponentLocation` (`self.LadderBottom`))))
      (`self.K2_SetActorLocation` (`self.BpPlayer`) (`KismetMathLibrary.VLerp` (`self.StartActorLocation`) _output_get _newtrack_0) false false))
    (:`Finished`
      (`self.Reset Player Y Pos` :!label _label)
      (set `self.bHasInteracted` false))))

(event `TimeLineReverse`
  (bind (_direction _newtrack_0) (`Timeline|Timeline` :!via `PlayFromStart`)
    (:`Update`
      (bind _output_get (set `self.EndActorLocation` (+ (0.0 0.0 100.0) (`SceneComponent.K2_GetComponentLocation` (`self.LadderTop`)))))
      (`self.K2_SetActorLocation` (`self.BpPlayer`) (`KismetMathLibrary.VLerp` (`self.StartActorLocation`) _output_get _newtrack_0) false false))
    (:`Finished`
      (goto _label))))

(event `Reset Player Y Pos`
  (bind _bpplayer (`self.BpPlayer`))
  (bind (_returnvalue_x _returnvalue_y _returnvalue_z) (`KismetMathLibrary.BreakVector` (`self.K2_GetActorLocation` _bpplayer)))
  (`self.K2_SetActorLocation` _bpplayer (`KismetMathLibrary.MakeVector` _returnvalue_x (`self.Player Starting Y Loc`) _returnvalue_z) false false))

(fn `Interact`
  (params (Interactor :type "Character Object Reference"))
  (returns (bSuccess :type Boolean))
  (bind (_returnvalue_x _returnvalue_y) (`KismetMathLibrary.BreakVector` (`self.K2_GetActorLocation` Interactor)))
  (`/Engine/EditorBlueprintResources/StandardMacros.IsValid` Interactor
    (:`Is Valid`
      (if (not (`self.bHasInteracted`))
        (set `self.Player Starting Y Loc` _returnvalue_y)
        (if (`PrimitiveComponent.IsOverlappingActor` (`self.TopCol`) Interactor)
          (bind _output_get (set `self.StartActorLocation` (`SceneComponent.K2_GetComponentLocation` (`self.LadderTop`))))
          (`self.K2_SetActorLocation` Interactor _output_get false false)
          (`self.TimeLineStart`)
          (set `self.bHasInteracted` true :!label _label)
          (return true)
          (elif (`PrimitiveComponent.IsOverlappingActor` (`self.BaseCol`) Interactor)
            (bind _output_get_2 (set `self.StartActorLocation` (`SceneComponent.K2_GetComponentLocation` (`self.LadderBottom`))))
            (`self.K2_SetActorLocation` Interactor _output_get_2 false false)
            (`self.TimeLineReverse`)
            (goto _label)))
        (else
          (return false))))
    (:`Is Not Valid`
      (return false))))

(fn `UserConstructionScript`)