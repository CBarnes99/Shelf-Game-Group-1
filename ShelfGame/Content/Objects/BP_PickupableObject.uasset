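; BP_PickupableObject is an actor for an object the player can pick up, switching its collision off while a player holds an item.
; BeginPlay caches player 0 into both ThisIsPlayer and PlayerTwo, so both reference the same character.
; Interact checks their IsItemHeld flag, sets collision to match and returns whether an item is held.
; Tick also updates collision from the BP_Player cast on overlap, without checking which item is held.
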(event `self.ReceiveBeginPlay`
  (bind _returnvalue (`GameplayStatics.GetPlayerCharacter` 0))
  (bind _asbp_player (cast `/Game/Characters/Player/BP_Player` _returnvalue))
  (set `self.ThisIsPlayer` _asbp_player)
  (bind _asbp_player_2 (cast `/Game/Characters/Player/BP_Player` _returnvalue))
  (set `self.PlayerTwo` _asbp_player_2))

(event `self.ReceiveActorBeginOverlap`
  (params (OtherActor :type "Actor Object Reference"))
  (bind _asbp_player (cast `/Game/Characters/Player/BP_Player` OtherActor))
  (set `self.ActorOverlap` true))

(event `self.ReceiveTick`
  (params (DeltaSeconds :type "Float (single-precision)"))
  (`/Engine/EditorBlueprintResources/StandardMacros.IsValid` (stale `self.ReceiveActorBeginOverlap` _asbp_player)
    (:`Is Valid`
      (if (`/Game/Characters/Player/BP_Player.IsItemHeld` (stale `self.ReceiveActorBeginOverlap` _asbp_player))
        (`self.SetActorEnableCollision` false)
        (else
          (`self.SetActorEnableCollision` true))))))

(fn `Interact`
  (params (Interactor :type "Character Object Reference"))
  (returns (bSuccess :type Boolean))
  (if (`/Game/Characters/Player/BP_Player.IsItemHeld` (`self.ThisIsPlayer`))
    (`self.SetActorEnableCollision` false)
    (elif (`/Game/Characters/Player/BP_Player.IsItemHeld` (`self.PlayerTwo`))
      (`self.SetActorEnableCollision` false)
      (else
        (`self.SetActorEnableCollision` true)
        (return false))))
  (return true))

(fn `UserConstructionScript`)