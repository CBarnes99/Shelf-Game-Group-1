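; Piccolina NPC Blueprint that adds a first-encounter cinematic and quest item count on top of its parent class.
; On BeginPlay it waits briefly, stores the number of quest sub-objectives as the amount of objects to receive, and prints a debug message.
; Interact plays the level sequence while HadFirstEncounter is false, then returns the parent's Interact result.
; The first-encounter flag is only read here, never set.
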(event `self.ReceiveBeginPlay`
  (`parent.ReceiveBeginPlay`)
  (`KismetSystemLibrary.Delay` 1.0)
  (set `self.Amount of Objects to Recieve` (`KismetArrayLibrary.Array_Length` (`/Game/Quests/ObjectiveTypes/BP_Objective_Collection.Sub Objectives` (`/Game/Quests/Quests/BP_BaseQuest.Objectives` (`self.Quest`)))))
  (`KismetSystemLibrary.PrintString` "Hello"))

(fn `Interact`
  (params (Interactor :type "Character Object Reference"))
  (returns (bSuccess :type Boolean))
  (if (not (`self.bHadFirstEncounter`))
    (`MovieSceneSequencePlayer.Play` (`LevelSequenceActor.SequencePlayer` (`self.LevelSequence`))))
  (bind _bsuccess (`parent.Interact` Interactor))
  (return _bsuccess))

(fn `UserConstructionScript`
  (`parent.UserConstructionScript`))