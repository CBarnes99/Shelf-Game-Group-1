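; BP_Emperor is an NPC that offers dialogue until its quest objectives are completed, then becomes an object the player can push and pivot.
; Interact starts the DialogueTree while the quest is unfinished, and afterwards enables AbleToPush on ACPushableObject, which BeginPlay leaves disabled.
; Push and pivot calls forward to that component only once the quest is complete, and a range check reports whether pushing is possible.
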(event `self.ReceiveBeginPlay`
  (`parent.ReceiveBeginPlay`)
  (set `/Game/ActorComponents/AC_PushableObject.AbleToPush` false (`self.AC_PushableObject`)))

(event `self.ReceiveTick`
  (params (DeltaSeconds :type "Float (single-precision)"))
  (`parent.ReceiveTick` DeltaSeconds))

(event `/Game/Interfaces/BPI_PushAndPivotCube.Push Object`
  (params (Direction :type "Float (double-precision)") (Player :type "Character Object Reference"))
  (if (`/Game/Quests/ObjectiveTypes/BP_Objective_Base.bIsCompleted` (`/Game/Quests/Quests/BP_BaseQuest.Objectives` (`self.Quest`)))
    (`/Game/ActorComponents/AC_PushableObject.Push Cube Called From Owner` (`self.AC_PushableObject`) Direction Player)))

(fn `Interact`
  (params (Interactor :type "Character Object Reference"))
  (returns (bSuccess :type Boolean))
  (`/Engine/EditorBlueprintResources/StandardMacros.IsValid` Interactor
    (:`Is Valid`
      (`KismetSystemLibrary.PrintString` (`KismetTextLibrary.Conv_TextToString` (`|FormatText` "Interacted with {this}" (`KismetSystemLibrary.GetObjectName` self))))
      (if (not (`/Game/Quests/ObjectiveTypes/BP_Objective_Base.bIsCompleted` (`/Game/Quests/Quests/BP_BaseQuest.Objectives` (`self.Quest`))))
        (`BrainComponent.StartLogic` (`self.Dialogue Tree`))
        (return true)
        (else
          (set `/Game/ActorComponents/AC_PushableObject.AbleToPush` true (`self.AC_PushableObject`))
          (`KismetSystemLibrary.PrintString` "Quest Finished, not showing dialogue")
          (return true))))
    (:`Is Not Valid`
      (`KismetSystemLibrary.PrintString` "Interactor Isn't Valid!")
      (return false))))

(fn `isPlayerInRangeAndAbleToPush`
  (returns (PlayerAbleToPush :type Boolean))
  (bind _ac_pushableobject (`self.AC_PushableObject`))
  (return (and (`/Game/ActorComponents/AC_PushableObject.PlayerInRange` _ac_pushableobject) (`/Game/ActorComponents/AC_PushableObject.AbleToPush` _ac_pushableobject))))

(fn `Pivot Object`
  (params (Direction :type "Float (double-precision)"))
  (returns (bSuccess :type Boolean))
  (if (`/Game/Quests/ObjectiveTypes/BP_Objective_Base.bIsCompleted` (`/Game/Quests/Quests/BP_BaseQuest.Objectives` (`self.Quest`)))
    (bind _bsuccess (`/Game/ActorComponents/AC_PushableObject.Pivot Object` (`self.AC_PushableObject`) Direction))
    (return _bsuccess)))

(fn `UserConstructionScript`
  (`parent.UserConstructionScript`))