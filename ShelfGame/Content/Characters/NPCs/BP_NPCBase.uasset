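; Base Blueprint for NPCs that starts dialogue when something interacts with the character.
; Interact validates the interactor, prints a debug message naming the NPC, calls StartLogic on DialogueTree and returns true.
; An invalid interactor prints an error and returns false.
; BeginPlay, overlap, Tick and the construction script contain no logic.
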(event `self.ReceiveBeginPlay`)

(fn `Interact`
  (params (Interactor :type "Character Object Reference"))
  (returns (bSuccess :type Boolean))
  (`/Engine/EditorBlueprintResources/StandardMacros.IsValid` Interactor
    (:`Is Valid`
      (`KismetSystemLibrary.PrintString` (`KismetTextLibrary.Conv_TextToString` (`|FormatText` "Interacted with {this}" (`KismetSystemLibrary.GetObjectName` self))))
      (`BrainComponent.StartLogic` (`self.Dialogue Tree`))
      (return true))
    (:`Is Not Valid`
      (`KismetSystemLibrary.PrintString` "Interactor Isn't Valid!")
      (return false))))

(fn `UserConstructionScript`)