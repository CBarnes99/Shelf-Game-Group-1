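; BP_NPC is an NPC that shows a floating name label when a character is nearby and can be interacted with.
; On BeginPlay it fills the text component from TrinketName and hides it; the naming suggests reuse from a trinket Blueprint.
; Box overlap events toggle the label for any Character, not only the player.
; Interact is a debug placeholder that validates the interactor, prints a message and returns success or failure.
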(event `self.ReceiveBeginPlay`
  (`self.Set Trinket Name`))

(event `self.Box.OnComponentBeginOverlap`
  (params (OverlappedComponent :type "PrimitiveComponent Object Reference") (OtherActor :type "Actor Object Reference") (OtherComp :type "PrimitiveComponent Object Reference") (OtherBodyIndex :type Integer) (bFromSweep :type Boolean) (SweepResult :type "HitResult Structure (by ref)"))
  (cast `Character` OtherActor)
  (`self.Set Name Visable` true))

(event `self.Box.OnComponentEndOverlap`
  (params (OverlappedComponent :type "PrimitiveComponent Object Reference") (OtherActor :type "Actor Object Reference") (OtherComp :type "PrimitiveComponent Object Reference") (OtherBodyIndex :type Integer))
  (cast `Character` OtherActor)
  (`self.Set Name Visable` false))

(fn `Interact`
  (params (Interactor :type "Character Object Reference"))
  (returns (bSuccess :type Boolean))
  (`/Engine/EditorBlueprintResources/StandardMacros.IsValid` Interactor
    (:`Is Valid`
      (`KismetSystemLibrary.PrintString` (`KismetTextLibrary.Conv_TextToString` (`|FormatText` "Interacted with {this}" (`KismetSystemLibrary.GetObjectName` self))))
      (return true))
    (:`Is Not Valid`
      (`KismetSystemLibrary.PrintString` "Interactor Isn't Valid!")
      (return false))))

(fn `Set Name Visable`
  (params (bIsPlayerByTrinket :type Boolean))
  (`SceneComponent.SetVisibility` (`self.Name of  Trinket`) bIsPlayerByTrinket false))

(fn `Set Trinket Name`
  (`TextRenderComponent.K2_SetText` (`self.Name of  Trinket`) (`self.Trinket Name`))
  (`SceneComponent.SetVisibility` (`self.Name of  Trinket`) false false))

(fn `UserConstructionScript`)