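; Core player controller that manages input and switches the player between 2D and 3D movement systems.
; On BeginPlay it fetches the core HUD, then on success adds the default and 2D Enhanced Input mapping contexts.
; ChangeMovementSystem swaps 2D for 3D plus mouse-look contexts, or back, and notifies the pawn through an interface.
; ToggleInput controls pawn input, cursor visibility and game-only or UI-only input mode.
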(event `self.ReceiveBeginPlay`
  (bind _returnvalue (subsystem `EnhancedInputLocalPlayerSubsystem`))
  (bind _bp_core_hud (`/Game/Macros/BML_PlayerController.Get_BP_Core_HUD` 10.0)
    (:`Success`
      (set `self.As BP Core HUD` _bp_core_hud)
      (`EnhancedInputSubsystemInterface.AddMappingContext` _returnvalue "/Game/Characters/Player/Input/IMC_Default.IMC_Default" 0 (struct))
      (`EnhancedInputSubsystemInterface.AddMappingContext` _returnvalue "/Game/Characters/Player/Input/IMC_2DMovement.IMC_2DMovement" 0 (struct)))
    (:`Failed`
      (`KismetSystemLibrary.PrintString` "Failed To Get Core HUD In Player Controller" true true (struct :`R` 1.0 :`B` 0.075243 :`A` 1.0) 100.0))))

(fn `2DMovement`
  (bind _returnvalue (subsystem `EnhancedInputLocalPlayerSubsystem`))
  (bind _returnvalue_2 (subsystem `EnhancedInputLocalPlayerSubsystem`))
  (if (`.ReturnValue` (`EnhancedInputSubsystemInterface.HasMappingContext` (subsystem `EnhancedInputLocalPlayerSubsystem`) "/Game/Characters/Player/Input/IMC_3DMovement.IMC_3DMovement"))
    (`EnhancedInputSubsystemInterface.RemoveMappingContext` _returnvalue "/Game/Characters/Player/Input/IMC_3DMovement.IMC_3DMovement" (struct))
    (`EnhancedInputSubsystemInterface.RemoveMappingContext` _returnvalue "/Game/Characters/Player/Input/IMC_MouseLook.IMC_MouseLook" (struct)))
  (if (not (`.ReturnValue` (`EnhancedInputSubsystemInterface.HasMappingContext` _returnvalue_2 "/Game/Characters/Player/Input/IMC_2DMovement.IMC_2DMovement")))
    (`EnhancedInputSubsystemInterface.AddMappingContext` _returnvalue_2 "/Game/Characters/Player/Input/IMC_2DMovement.IMC_2DMovement" 0 (struct))))

(fn `3DMovement`
  (bind _returnvalue (subsystem `EnhancedInputLocalPlayerSubsystem`))
  (if (`.ReturnValue` (`EnhancedInputSubsystemInterface.HasMappingContext` (subsystem `EnhancedInputLocalPlayerSubsystem`) "/Game/Characters/Player/Input/IMC_2DMovement.IMC_2DMovement"))
    (`EnhancedInputSubsystemInterface.RemoveMappingContext` (subsystem `EnhancedInputLocalPlayerSubsystem`) "/Game/Characters/Player/Input/IMC_2DMovement.IMC_2DMovement" (struct)))
  (if (not (`.ReturnValue` (`EnhancedInputSubsystemInterface.HasMappingContext` _returnvalue "/Game/Characters/Player/Input/IMC_3DMovement.IMC_3DMovement")))
    (`EnhancedInputSubsystemInterface.AddMappingContext` _returnvalue "/Game/Characters/Player/Input/IMC_3DMovement.IMC_3DMovement" 0 (struct))
    (`EnhancedInputSubsystemInterface.AddMappingContext` _returnvalue "/Game/Characters/Player/Input/IMC_MouseLook.IMC_MouseLook" 0 (struct))))

(fn `ChangeMovementSystem`
  (params (`Movement System` :type "/Game/Characters/Player/StateEnums/E_MovementSystem Enum" :default "NewEnumerator0"))
  (bind _returnvalue (`GameplayStatics.GetPlayerPawn` 0))
  (switch `/Game/Characters/Player/StateEnums/E_MovementSystem` `Movement System`
    (:`NewEnumerator0`
      (`self.2DMovement`))
    (:`NewEnumerator1`
      (`self.3DMovement`)))
  (if (`KismetSystemLibrary.DoesImplementInterface` _returnvalue "/Game/Interfaces/BPI_UpdatePlayerMovementSystem.BPI_UpdatePlayerMovementSystem_C")
    (bind _new_movement_system (message `/Game/Interfaces/BPI_UpdatePlayerMovementSystem.Update Movement System` _returnvalue `Movement System`))
    (`KismetSystemLibrary.PrintString` (`KismetTextLibrary.Conv_TextToString` (`|FormatText` "New Movement System = {Movement System}" (`|GetEnumeratorNameAsString` _new_movement_system))))
    (else
      (`KismetSystemLibrary.PrintString` (`KismetTextLibrary.Conv_TextToString` (`|FormatText` "{Player Pawn} doenst have BPI Update Player Movement System Interface " (`GameplayStatics.GetPlayerPawn` 0))) true true (struct :`R` 1.0 :`G` 0.000211 :`A` 1.0) 10.0))))

(fn `Toggle Input`
  (params (bEnableInput :type Boolean) (bFocusGame :type Boolean))
  (returns (bInputIsEnabled :type Boolean) (bGameIsInFocus :type Boolean))
  (locals (bIsInputEnabled :type Boolean) (bIsGameInFocus :type Boolean))
  (if bEnableInput
    (`self.EnableInput` (`self.K2_GetPawn`) self)
    (set `local.bIsInputEnabled` true)
    (else
      (`self.StopMovement` self)
      (`self.DisableInput` (`self.K2_GetPawn`) self)))
  (if bFocusGame
    (set `self.bShowMouseCursor` false)
    (`WidgetBlueprintLibrary.SetInputMode_GameOnly` self)
    (set `local.bIsGameInFocus` true)
    (else
      (set `self.bShowMouseCursor` true)
      (`WidgetBlueprintLibrary.SetInputMode_UIOnlyEx` self null)))
  (return (`local.bIsInputEnabled`) (`local.bIsGameInFocus`)))

(fn `UserConstructionScript`)