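; Core HUD that manages on-screen menu widgets and switches input between game and UI.
; BeginPlay sets game-only input, then adds the game menu, menu and modal widget lists to the viewport collapsed.
; Toggling a game menu collapses the others, then shows it with Game-and-UI input and cursor, or hides it and restores game input.
; NPC dialogue toggle is a placeholder, and its widget creation is disconnected, so never runs.
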(event `self.ReceiveBeginPlay`
  (bind _output_get (set `self.Player Controller` (`self.GetOwningPlayerController`)))
  (`WidgetBlueprintLibrary.SetInputMode_GameOnly` _output_get)
  (`|ExecutionSequence`
    (:`then_4`
      ; Collapse all non Game Widgets created widgets
      (`self.Collapse Widgets` (`self.Game Menu Widgets List`))
      (`self.Collapse Widgets` (`self.Menu Widgets List`))
      (`self.Collapse Widgets` (`self.Modal Widgets List`)))))

(event `Toggle NPC Dialogue`
  ; PLACEHOLDER! Called From Player Controller
  (`KismetSystemLibrary.PrintString` "Toggle NPC Dialogue")
  (`self.Toggle Game Menu Widgets` (`self.NPC Dialogue`)))

(fn `Collapse Widgets`
  (params (`Widget Array` :type "Array of UserWidget Object Reference"))
  (for _array_element `Widget Array`
    (`UserWidget.AddToViewport` _array_element 0)
    (`Widget.SetVisibility` _array_element "Collapsed")))

(fn `Focus Game`
  (bind _player_controller (`self.Player Controller`))
  (`Widget.SetVisibility` (`self.Widget To Focus`) "Collapsed")
  (`WidgetBlueprintLibrary.SetInputMode_GameOnly` _player_controller)
  (set `PlayerController.bShowMouseCursor` false _player_controller))

(fn `Focus Widget`
  (`Widget.SetVisibility` (`self.Widget To Focus`) "SelfHitTestInvisible")
  (`WidgetBlueprintLibrary.SetInputMode_GameAndUIEx` (`self.Player Controller`) (`self.Widget To Focus`))
  (set `PlayerController.bShowMouseCursor` true (`self.Player Controller`)))

(fn `Toggle Game Menu Widgets`
  (params (`Target Widget` :type "UserWidget Object Reference"))
  (`/Engine/EditorBlueprintResources/StandardMacros.IsValid` `Target Widget`
    (:`Is Valid`
      (set `self.Widget To Focus` `Target Widget`)
      (for _array_element (`self.Game Menu Widgets List`)
        (`/Engine/EditorBlueprintResources/StandardMacros.IsValid` _array_element
          (:`Is Valid`
            (if (== (`self.Widget To Focus`) _array_element)
              (if (`Widget.IsVisible` (`self.Widget To Focus`))
                (`self.Focus Game`)
                (else
                  (`self.Focus Widget`)))
              (elif (`Widget.IsVisible` _array_element)
                (`Widget.SetVisibility` _array_element "Collapsed")))))))
    (:`Is Not Valid`
      (`KismetSystemLibrary.PrintString` "Focusing Widget Not Valid"))))

(fn `UserConstructionScript`)