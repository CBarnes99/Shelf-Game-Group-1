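; Base actor for arm pickups that attach to a character and carry an ability.
; PickupArm works once, snapping the arm to a given socket on the interactor's mesh and disabling Cube collision if attachment succeeds.
; It then returns success, the arm, and its ability and tag to the caller.
; Interact is a stub returning false, and the event graph and construction script are empty.
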(fn `Interact`
  (params (Interactor :type "Character Object Reference"))
  (returns (bSuccess :type Boolean))
  (return false))

(fn `PickupArm`
  (params (Interactor :type "Character Object Reference") (`Socket To Attach To` :type Name))
  (returns (bSuccess :type Boolean) (Arm :type "/Game/Arms/ArmActors/BP_ArmsBase Object Reference") (`Ability Tag` :type "GameplayTagContainer Structure") (Ability :type "GameplayAbility Class Reference"))
  (if (not (`self.Has Been Picked Up`))
    (bind _returnvalue (`self.K2_AttachToComponent` (`Character.Mesh` Interactor) `Socket To Attach To` "SnapToTarget" "SnapToTarget" "SnapToTarget"))
    (bind _output_get (set `self.Has Been Picked Up` _returnvalue))
    (if _output_get
      (`PrimitiveComponent.SetCollisionEnabled` (`self.Cube`) "NoCollision"))
    (return _output_get self (`self.Ability Tag`) (`self.Ability`))))

(fn `UserConstructionScript`)