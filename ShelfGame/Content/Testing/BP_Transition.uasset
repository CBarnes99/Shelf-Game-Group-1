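; BP_Transition is an interactable teleporter in the Testing folder that moves an actor to a linked transition actor.
; On BeginPlay it caches its Cube's world location as TeleportLocation.
; Interact teleports a valid Interactor to the linked TransitionActor's TeleportLocation and returns success, otherwise it prints an error and returns false.
; The CollisionBox overlap event is empty, and its Player-tag teleport logic is disconnected, so only Interact triggers travel.
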(event `self.ReceiveBeginPlay`
  (set `self.Teleport Location` (`SceneComponent.K2_GetComponentLocation` (`self.Cube`))))

(event `self.CollisionBox.OnComponentBeginOverlap`
  (params (OverlappedComponent :type "PrimitiveComponent Object Reference") (OtherActor :type "Actor Object Reference") (OtherComp :type "PrimitiveComponent Object Reference") (OtherBodyIndex :type Integer) (bFromSweep :type Boolean) (SweepResult :type "HitResult Structure (by ref)")))

(fn `Interact`
  (params (Interactor :type "Character Object Reference"))
  (returns (bSuccess :type Boolean))
  (`/Engine/EditorBlueprintResources/StandardMacros.IsValid` Interactor
    (:`Is Valid`
      (`self.K2_SetActorLocation` Interactor (`/Game/Testing/BP_Transition.Teleport Location` (`self.Transition Actor`)) false true)
      (return true))
    (:`Is Not Valid`
      (`KismetSystemLibrary.PrintString` "Interactor Isn't Valid!")
      (return false))))

(fn `UserConstructionScript`)