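; BP_Cable is a test actor for an interactable cable, with only debug behavior so far.
; Interact checks for a valid interactor and that HasBeenCut is false, then prints the Cable component's world location and EndLocation and returns true.
; An invalid interactor prints a warning and returns false; nothing here performs the cut.
; PickupArm always reports failure, and the event graph and construction script are empty.
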(fn `Interact`
  (params (Interactor :type "Character Object Reference"))
  (returns (bSuccess :type Boolean))
  (bind _cable (`self.Cable`))
  (`/Engine/EditorBlueprintResources/StandardMacros.IsValid` Interactor
    (:`Is Valid`
      (if (not (`self.bHasBeenCut`))
        (`KismetSystemLibrary.PrintString` (`KismetTextLibrary.Conv_TextToString` (`|FormatText` "World loc {loc}" (`KismetStringLibrary.Conv_VectorToString` (`SceneComponent.K2_GetComponentLocation` _cable)))))
        (`KismetSystemLibrary.PrintString` (`KismetTextLibrary.Conv_TextToString` (`|FormatText` "End Loc {loc}" (`KismetStringLibrary.Conv_VectorToString` (`CableComponent.EndLocation` _cable)))))
        (return true)))
    (:`Is Not Valid`
      (`KismetSystemLibrary.PrintString` "Interactor Not Valid On Cable" true true (struct :`R` 1.0 :`G` 0.076353 :`A` 1.0) 2.01)
      (return false))))

(fn `PickupArm`
  (params (Interactor :type "Character Object Reference") (`Socket To Attach To` :type Name))
  (returns (bSuccess :type Boolean) (Arm :type "/Game/Tools/ToolActors/BP_ToolsBase Object Reference") (`Ability Tag` :type "GameplayTagContainer Structure") (Ability :type "GameplayAbility Class Reference"))
  (return false null (struct) null))

(fn `UserConstructionScript`)