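; BP_CutsceneTriggerBox is a one-shot trigger volume that starts a cutscene when the player enters its box.
; On BeginPlay it finds the BP_CutsceneManager and binds to its cutscene-finished event, destroying itself if none exists.
; A Player-tagged overlap passes a data table row name to the manager and sets IsActive, blocking retriggers.
; When a cutscene ends while it is active, it unbinds and destroys itself.
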(event `self.ReceiveBeginPlay`
  (bind _returnvalue (`GameplayStatics.GetActorOfClass` "/Game/Cutscenes/BP_CutsceneManager.BP_CutsceneManager_C"))
  (`/Engine/EditorBlueprintResources/StandardMacros.IsValid` _returnvalue
    (:`Is Valid`
      (bind _output_get (set `self.CutsceneManager` _returnvalue))
      (add `/Game/Cutscenes/BP_CutsceneManager.CurrentCutsceneFinished` _output_get (`|CreateDelegate` :!event `Cutscene Ended`)))
    (:`Is Not Valid`
      (`KismetSystemLibrary.PrintString` "Cutscene Manager Not Valid!")
      (`self.K2_DestroyActor`))))

(event `self.Box.OnComponentBeginOverlap`
  (params (OverlappedComponent :type "PrimitiveComponent Object Reference") (OtherActor :type "Actor Object Reference") (OtherComp :type "PrimitiveComponent Object Reference") (OtherBodyIndex :type Integer) (bFromSweep :type Boolean) (SweepResult :type "HitResult Structure (by ref)"))
  (if (and (`self.ActorHasTag` OtherActor "Player") (not (`self.bIsActive`)))
    (`/Game/Cutscenes/BP_CutsceneManager.PlayCutscene` (`self.CutsceneManager`) (`self.Cutscene DataTable Row Name`))
    (set `self.bIsActive` true)))

(event `Cutscene Ended`
  (if (`self.bIsActive`)
    (remove `/Game/Cutscenes/BP_CutsceneManager.CurrentCutsceneFinished` (`self.CutsceneManager`) (delegate `Cutscene Ended`))
    (`self.K2_DestroyActor`)))

(fn `UserConstructionScript`)