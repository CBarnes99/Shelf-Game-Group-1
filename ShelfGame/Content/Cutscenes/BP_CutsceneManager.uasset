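; BP_CutsceneManager plays image-based cutscenes from DT_Cutscenes, looked up by row name.
; PlayCutscene creates a WBP_Cutscene with the row's images, plays its open animation, and sends a controller message disabling input and showing the mouse; missing rows print an error.
; When the widget ends, CutsceneFinished fires the CurrentCutsceneFinished dispatcher, removes the widget and restores input.
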(event `PlayCutscene`
  (params (CutsceneRowName :type Name))
  (bind _returnvalue (`|GetDataTableRow` "/Game/Cutscenes/Widgets/DT_Cutscenes.DT_Cutscenes" CutsceneRowName)
    (:`then`
      (bind _returnvalue_2 (`|CreateWidget` "/Game/Cutscenes/Widgets/WBP_Cutscene.WBP_Cutscene_C" null (`.CutsceneImages_3_12291A8F436853AFB84665BF78605B01` (break `/Game/Cutscenes/Widgets/F_Cutscenes` _returnvalue))))
      (bind _output_get (set `self.Cutscene` _returnvalue_2))
      (add `/Game/Cutscenes/Widgets/WBP_Cutscene.Cutscene Ended` _output_get (`|CreateDelegate` :!event `CutsceneFinished`))
      (`UserWidget.AddToViewport` _output_get 0)
      (`/Game/Cutscenes/Widgets/WBP_Cutscene.Play Open Animation` _output_get)
      (message `/Game/Interfaces/BPI_ToggleInputForDialogue.Toggle Input` (`GameplayStatics.GetPlayerController` 0) false false true))
    (:`RowNotFound`
      (`KismetSystemLibrary.PrintString` (`KismetTextLibrary.Conv_TextToString` (`|FormatText` "Cutscene DataTable Row Name Not Found - {Name}" CutsceneRowName)) true true (struct :`R` 1.0 :`G` 0.031773 :`A` 1.0) 15.0))))

(event `CutsceneFinished`
  (bind _cutscene (`self.Cutscene`))
  (`self.CurrentCutsceneFinished`)
  (clear `/Game/Cutscenes/Widgets/WBP_Cutscene.Cutscene Ended` _cutscene)
  (`Widget.RemoveFromParent` _cutscene)
  (message `/Game/Interfaces/BPI_ToggleInputForDialogue.Toggle Input` (`GameplayStatics.GetPlayerController` 0) true true false))

(fn `UserConstructionScript`)