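; BP_Cutscene is an interactable actor that plays a cutscene built from its list of textures.
; Interacting creates a WBP_Cutscene widget with those textures, adds it to the viewport, and switches player controller 0 from game input to mouse via ToggleInputMessage.
; The widget's CutsceneEnded event is bound on start; CutsceneFinished unbinds it, removes the widget and restores game input.
; An empty texture list only prints an error.
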(event `Start Cutscene`
  (bind _returnvalue (`GameplayStatics.GetPlayerController` 0))
  (bind _cutscene_textures (`self.Cutscene Textures`))
  (if (`KismetArrayLibrary.Array_IsValidIndex` _cutscene_textures)
    (bind _returnvalue_2 (`|CreateWidget` "/Game/Cutscenes/Widgets/WBP_Cutscene.WBP_Cutscene_C" _returnvalue _cutscene_textures))
    (set `self.Cutscene Widget` _returnvalue_2)
    (add `/Game/Cutscenes/Widgets/WBP_Cutscene.Cutscene Ended` _returnvalue_2 (`|CreateDelegate` :!event `Cutscene Finished`))
    (`UserWidget.AddToViewport` _returnvalue_2 0)
    (message `/Game/Interfaces/BPI_ToggleInputForDialogue.Toggle Input` _returnvalue false false true)
    (else
      (`KismetSystemLibrary.PrintString` "No valid textures in cutscene actor!!!" true true (struct :`R` 1.0 :`B` 0.070465 :`A` 1.0) 10.0))))

(event `Cutscene Finished`
  (bind _cutscene_widget (`self.Cutscene Widget`))
  (clear `/Game/Cutscenes/Widgets/WBP_Cutscene.Cutscene Ended` _cutscene_widget)
  (`Widget.RemoveFromParent` _cutscene_widget)
  (message `/Game/Interfaces/BPI_ToggleInputForDialogue.Toggle Input` (`GameplayStatics.GetPlayerController` 0) true true false))

(fn `Interact`
  (params (Interactor :type "Character Object Reference"))
  (returns (bSuccess :type Boolean))
  (`/Engine/EditorBlueprintResources/StandardMacros.IsValid` Interactor
    (:`Is Valid`
      (`self.Start Cutscene`)
      (return true))
    (:`Is Not Valid`
      (return false))))

(fn `UserConstructionScript`)