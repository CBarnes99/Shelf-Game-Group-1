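; Crafting bench actor that turns Tin placed by the player into crafted items through a jigsaw puzzle mini game.
; Interact takes held Tin and attaches it to a mesh socket.
; CraftItem, meant for hammer use, opens a puzzle widget configured by the current JigsawPuzzleElements entry and switches input to mouse.
; On completion, the bench replaces the Tin with that entry's spawned object, restores game input and advances the index until entries run out.
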(event `Puzzle Finished`
  ; When the puzzle is finished, spawn the crafted item
  (`self.K2_DestroyActor` (`self.ItemOnBench`))
  (bind _returnvalue (`|SpawnActorFromClass` (`.ObjectToSpawn_19_23C205F74EBEBF8EE976299CD2E8B062` (break `/Game/F_JigsawPuzzleElemets` (`|GetArrayItem` (`self.Jigsaw Puzzle Elements`) (`self.Puzzle Index`)))) (`KismetMathLibrary.MakeTransform` (0.0 0.0 0.0)) "Undefined" "MultiplyWithRoot" null null))
  (`self.K2_AttachToComponent` _returnvalue (`self.StaticMesh`) (`self.Socket To Attach To`) "KeepRelative" "KeepRelative" "KeepRelative" true)
  (`/Engine/EditorBlueprintResources/StandardMacros.IncrementInt` (`self.Puzzle Index`)
    (:`  `
      (`Widget.RemoveFromParent` (`self.Current Puzzle`))
      (message `/Game/Interfaces/BPI_ToggleInputForDialogue.Toggle Input` (`GameplayStatics.GetPlayerController` 0) true true false)
      (`/Game/ActorComponents/AC_InteractAsText.Reset Widget` (`self.AC_InteractAndAbilityAsText`)))))

(fn `Craft Item`
  (returns (bSuccess :type Boolean))
  (bind _jigsaw_puzzle_elements (`self.Jigsaw Puzzle Elements`))
  (bind (_thingtosmash _amounttoclick _numberofjigsawpieces _puzzleimage _jigsawpiecesize) (break `/Game/F_JigsawPuzzleElemets` (`|GetArrayItem` _jigsaw_puzzle_elements (`self.Puzzle Index`))))
  ; If Interacted with by the player using a Hammer, start the puzzle mini game
  (`self.ItemOnBench`
    (:`then`
      (if (< (`self.Puzzle Index`) (`KismetArrayLibrary.Array_Length` _jigsaw_puzzle_elements))
        (bind _returnvalue (`|CreateWidget` "/Game/Widgets/JigsawPuzzle/WBP_JigsawPuzzle.WBP_JigsawPuzzle_C" null _thingtosmash _amounttoclick _numberofjigsawpieces _puzzleimage _jigsawpiecesize))
        (set `self.Current Puzzle` _returnvalue)
        (`UserWidget.AddToViewport` _returnvalue 0)
        (add `/Game/Widgets/JigsawPuzzle/WBP_JigsawPuzzle.Puzzle Completed` _returnvalue (`|CreateDelegate` :!event `Puzzle Finished`))
        (message `/Game/Interfaces/BPI_ToggleInputForDialogue.Toggle Input` (`GameplayStatics.GetPlayerController` 0) false false true)
        (`/Game/ActorComponents/AC_InteractAsText.Reset Widget` (`self.AC_InteractAndAbilityAsText`))
        (return true)
        (else
          (`KismetSystemLibrary.PrintString` "Have Exhausted All Jigsaw Puzzle Elemts within Crafting Bench")
          (return false))))
    (:`else`
      (`KismetSystemLibrary.PrintString` "No Item On Bench")
      (return false))))

(fn `Interact`
  (params (Interactor :type "Character Object Reference"))
  (returns (bSuccess :type Boolean))
  ; If the player is holding an object that is Tin, Attach that to the bench
  (`/Engine/EditorBlueprintResources/StandardMacros.IsValid` Interactor
    (:`Is Valid`
      (`self.ItemOnBench`
        (:`then`)
        (:`else`
          (bind (_bsuccess _held_object) (message `/Game/Interfaces/BPI_GetFromPlayer.Get Held Object` Interactor))
          (if _bsuccess
            (`KismetSystemLibrary.IsObjectOfSoftClass` _held_object "/Game/Objects/Pickup-able_Actors/BP_Pickup_Tin.BP_Pickup_Tin_C"
              (:`True`
                (set `self.ItemOnBench` _held_object)
                (message `/Game/Interfaces/BPI_GetFromPlayer.Remove Held Object` Interactor false)
                (`self.K2_AttachToComponent` (`self.ItemOnBench`) (`self.StaticMesh`) (`self.Socket To Attach To`) "SnapToTarget" "SnapToTarget" "SnapToTarget" true)
                (`self.SetActorEnableCollision` (`self.ItemOnBench`) false)
                (`/Game/ActorComponents/AC_InteractAsText.Reset Widget` (`self.AC_InteractAndAbilityAsText`)))
              (:`False`
                (`KismetSystemLibrary.PrintString` "Held Object Isn't Tin")
                (return false)))
            (else
              (`KismetSystemLibrary.PrintString` "Player Has No Held Item")
              (return false))))))
    (:`Is Not Valid`
      (`KismetSystemLibrary.PrintString` "Interactor Not Valid")
      (return false))))

(fn `UserConstructionScript`)